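; BP_Socket is a socket client actor in the LLM folder that sends text to a server at a given IP and port.
; StablishConnection opens the connection, registers delegates and stores the connection ID used by SendMessage to send text as bytes.
; InitializeInputWidget stores an input widget and binds a delegate to its send-text event.
; The connected, disconnected and message-received events are empty, so replies go unhandled here.
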(event `self.ReceiveBeginPlay`)

(event `onConnected`
  (params (ConnectionId :type Integer)))

(event `onDisconnected`
  (params (ConnectionId :type Integer)))

(event `onMessageReceived`
  (params (ConnectionId :type Integer) (Message :type "Array of Byte (by ref)")))

(fn `InitializeInputWidget`
  (params (InputWidgetParam :type "/Game/Game/Blueprints/LLM/WBP_TutorialBuddyInputPanel Object Reference"))
  (bind _output_get (set `self.InputWidget` InputWidgetParam))
  (add `/Game/Game/Blueprints/LLM/WBP_TutorialBuddyInputPanel.onSendText` _output_get (`|CreateDelegate` :!event `Send Message`)))

(fn `Send Message`
  (params (Text :type Text))
  (`self.SendData` (`self.ServerConnectionId`) (`self.Conv_StringToBytes` (`KismetTextLibrary.Conv_TextToString` Text))))

(fn `StablishConnection`
  (params (IP_Param :type String) (Port_Param :type Integer))
  (bind _output_get (set `self.IP` IP_Param))
  (bind _output_get_2 (set `self.Port` Port_Param))
  (bind _connectionid (`self.Connect` _output_get _output_get_2 (`|CreateDelegate` :!event `onDisconnected`) (`|CreateDelegate` :!event `onConnected`) (`|CreateDelegate` :!event `onMessageReceived`)))
  (set `self.ServerConnectionId` _connectionid))

(fn `UserConstructionScript`)