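; BP_MessageBuilder is an Actor that builds JSON messages, apparently for the game's LLM communication.
; BuildQuestionMessage adds a question type and its text to the supplied JSON, while BuildSyncMessage adds a sync type.
; Both pass through BuildData, which appends a data object with hardcoded test name and age fields, plus a formatted timestamp from the current time.
; It only assembles and returns messages, with no event logic or sending.
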(fn `BuildData`
  (params (Json :type "BlueprintJsonObject Structure"))
  (returns (JsonData :type "BlueprintJsonObject Structure"))
  (bind (_year _month _day _hour _minute _second _millisecond) (`KismetMathLibrary.BreakDateTime` (`KismetMathLibrary.Now`)))
  (return (`BlueprintJsonLibrary.JsonMakeField` (`BlueprintJsonLibrary.JsonMakeField` Json "data" (`BlueprintJsonLibrary.JsonMakeObject` (`BlueprintJsonLibrary.JsonMakeField` (`BlueprintJsonLibrary.JsonMakeField` (`BlueprintJsonLibrary.JsonMake`) "Nombre" (`BlueprintJsonLibrary.JsonMakeString` "NombrePrueba")) "Edad" (`BlueprintJsonLibrary.JsonMakeInt` 30)))) "timestamp" (`BlueprintJsonLibrary.JsonMakeString` (`KismetStringLibrary.Replace` (`KismetTextLibrary.Conv_TextToString` (`|FormatText` "{Ano}/{Mes}/{Dia}_{Hora}:{Minuto}:{Segundo}.{Milisegundo}" (`KismetStringLibrary.Conv_IntToString` _year) _month _day _hour _minute _second _millisecond)) " ")))))

(fn `BuildQuestionMessage`
  (params (Question :type Text) (Json :type "BlueprintJsonObject Structure"))
  (returns (JsonQuestion :type "BlueprintJsonObject Structure"))
  (bind _jsondata (`self.BuildData` (`BlueprintJsonLibrary.JsonMakeField` (`BlueprintJsonLibrary.JsonMakeField` Json "type" (`BlueprintJsonLibrary.JsonMakeString` "question")) "text" (`BlueprintJsonLibrary.JsonMakeString` (`KismetTextLibrary.Conv_TextToString` Question)))))
  (return _jsondata))

(fn `BuildSyncMessage`
  (params (Json :type "BlueprintJsonObject Structure"))
  (returns (JsonQuestion :type "BlueprintJsonObject Structure"))
  (bind _jsondata (`self.BuildData` (`BlueprintJsonLibrary.JsonMakeField` Json "type" (`BlueprintJsonLibrary.JsonMakeString` "sync"))))
  (return _jsondata))

(fn `UserConstructionScript`)