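; BP_LLM_Manager runs the tutorial buddy's question input and relays messages to a local LLM socket endpoint.
; StartLLM creates the input panel, spawns socket and message-builder actors, binds question submission, and connects to localhost.
; ManageQuestion and ManageSync send builder-made JSON as strings through the socket, with questions also closing the panel.
; BeginPlay starts a looping timer and enables input so T toggles the panel.
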(event `self.ReceiveBeginPlay`
  (`KismetSystemLibrary.K2_SetTimerDelegate` (`|CreateDelegate` :!event `ManageSync`) 10.0 true)
  (`self.EnableInput` (`GameplayStatics.GetPlayerController` 0)))

(event `Key|T`
  (params (Key :type "Key Structure"))
  (:`Pressed`
    (if (`self.isInputDialogVisible`)
      (`self.Hide Input Dialog`)
      (else
        (`self.ShowInputDialog`)))))

(fn `Hide Input Dialog`
  (`Widget.RemoveFromParent` (`self.InputDialog`))
  (set `self.isInputDialogVisible` false))

(fn `ManageQuestion`
  (params (Text :type Text))
  (bind _jsonquestion (`/Game/Game/Blueprints/LLM/BP_MessageBuilder.BuildQuestionMessage` (`self.MessageBuilder`) Text (`BlueprintJsonLibrary.JsonMake`)))
  (`/Game/Game/Blueprints/LLM/BP_Socket.Send Message` (`self.Socket`) (`BlueprintJsonLibrary.Conv_JsonObjectToString` _jsonquestion))
  (`self.Hide Input Dialog`))

(fn `ManageSync`
  (bind _jsonquestion (`/Game/Game/Blueprints/LLM/BP_MessageBuilder.BuildSyncMessage` (`self.MessageBuilder`) (`BlueprintJsonLibrary.JsonMake`)))
  (`/Game/Game/Blueprints/LLM/BP_Socket.Send Message` (`self.Socket`) (`BlueprintJsonLibrary.Conv_JsonObjectToString` _jsonquestion)))

(fn `ShowInputDialog`
  (`UserWidget.AddToViewport` (`self.InputDialog`) 0)
  (`WidgetBlueprintLibrary.SetInputMode_GameAndUIEx` (`GameplayStatics.GetPlayerController` 0) null)
  (set `self.isInputDialogVisible` true))

(fn `StartLLM`
  (`|ExecutionSequence`
    (:`then_0`
      (bind _returnvalue (`|CreateWidget` "/Game/Game/Blueprints/LLM/WBP_TutorialBuddyInputPanel.WBP_TutorialBuddyInputPanel_C"))
      (set `self.InputDialog` _returnvalue)
      (bind _returnvalue_2 (`|SpawnActorFromClass` "/Game/Game/Blueprints/LLM/BP_Socket.BP_Socket_C" (`KismetMathLibrary.MakeTransform` (0.0 0.0 0.0)) "Undefined" "MultiplyWithRoot" null null))
      (bind _output_get (set `self.Socket` _returnvalue_2))
      (set `/Game/Game/Blueprints/LLM/BP_Socket.InputWidget` (`self.InputDialog`) _output_get)
      (bind _returnvalue_3 (`|SpawnActorFromClass` "/Game/Game/Blueprints/LLM/BP_MessageBuilder.BP_MessageBuilder_C" (`KismetMathLibrary.MakeTransform` (0.0 0.0 0.0)) "Undefined" "MultiplyWithRoot" null null))
      (set `self.MessageBuilder` _returnvalue_3))
    (:`then_1`
      (`WidgetBlueprintLibrary.SetInputMode_GameAndUIEx` (`GameplayStatics.GetPlayerController` 0) null)
      (set `self.isInputDialogVisible` false))
    (:`then_2`
      (add `/Game/Game/Blueprints/LLM/WBP_TutorialBuddyInputPanel.onCommitedQuestion` (`self.InputDialog`) (`|CreateDelegate` :!event `ManageQuestion`)))
    (:`then_3`
      (`/Game/Game/Blueprints/LLM/BP_Socket.StablishConnection` (`self.Socket`) "127.0.0.1" 65431))))

(fn `UserConstructionScript`)