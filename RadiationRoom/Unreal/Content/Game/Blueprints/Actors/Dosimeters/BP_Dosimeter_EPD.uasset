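; Electronic personal dosimeter (EPD) actor that displays radiation dose rate and absorption on a widget and interacts via the player's left hand.
; BeginPlay derives an ID from the EPD count, registers with the gameplay manager and starts a self-recalling half-second update loop.
; When an emission point exists, each update buffers readings, location and time.
; ACDatabase sends them every ten samples or on the last-events flush, then the buffers clear.
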(event `self.ReceiveBeginPlay`
  (bind _gameplaymanager (`/Game/Game/FunctionLibraries/BFL_Common.GetMyGameplayManager`))
  (`parent.ReceiveBeginPlay`)
  (`|ExecutionSequence`
    (:`then_0`
      (`self.SetEPDId`)
      (bind _aswbp_dosimeter_for_dose_and_absortion_radiation_rate (cast `/Game/Game/UserInterfaces/Items/Dosimeters/WBP_DosimeterForDoseAndAbsortionRadiationRate` (`WidgetComponent.GetWidget` (`self.RadiationInfoWidgetComponent`))))
      (set `self.RadiationInfoWidgetActor` _aswbp_dosimeter_for_dose_and_absortion_radiation_rate)
      (`self.ShowRadiation`))
    (:`then_1`
      (`/Engine/EditorBlueprintResources/StandardMacros.IsValid` _gameplaymanager
        (:`Is Valid`
          (`/Game/Game/Blueprints/Gameplay/BP_GameplayManager.AddItemToGameManagerImportantList` _gameplaymanager (`self.ItemType`) self))))))

(event `self.ReceiveTick`
  (params (DeltaSeconds :type "Float (single-precision)"))
  (`parent.ReceiveTick` DeltaSeconds))

(event `/Game/Game/Interfaces/BI_ItemInteract.InteractWith`
  (params (Player :type "/Game/Game/Blueprints/Player/BP_Player Object Reference") (Hand :type "EControllerHand Enum" :default "Left"))
  (`parent.InteractWith` Player "Left"))

(event `ShowRadiation`
  (bind _ac_radiation (`self.AC_Radiation`))
  (`/Game/Game/UserInterfaces/Items/Dosimeters/WBP_DosimeterForDoseAndAbsortionRadiationRate.SetRadiationRate` (`self.RadiationInfoWidgetActor`) (`/Game/Game/Components/AC_Radiation.DoseRate` _ac_radiation) (`/Game/Game/Components/AC_Radiation.DoseAbsorption` _ac_radiation))
  (`self.SendEPDRadiationEventToDB`)
  (`KismetSystemLibrary.Delay` 0.5)
  (`self.ShowRadiation`))

(event `SendEPDRadiationEventToDB`
  (bind _ac_radiation (`self.AC_Radiation`))
  (bind _returnvalue (`GameplayStatics.GetActorOfClass` "/Game/Game/Blueprints/Actors/Radiation/BP_RadiationEmissionPoint.BP_RadiationEmissionPoint_C"))
  (`/Engine/EditorBlueprintResources/StandardMacros.IsValid` _returnvalue
    (:`Is Valid`
      (`KismetArrayLibrary.Array_Add` (`self.CurrentEventDoseRateArray`) (`/Game/Game/Components/AC_Radiation.DoseRate` _ac_radiation))
      (`KismetArrayLibrary.Array_Add` (`self.CurrentEventDoseAbsortionArray`) (`/Game/Game/Components/AC_Radiation.DoseAbsorption` _ac_radiation))
      (`KismetArrayLibrary.Array_Add` (`self.CurrentEventPositionArray`) (`self.K2_GetActorLocation`))
      (bind _returnvalue_2 (`KismetArrayLibrary.Array_Add` (`self.CurrentEventDatetimeArray`) (`KismetMathLibrary.Now`)))
      (if (>= _returnvalue_2 9)
        (`self.SendEventToDB`)))))

(event `SendEventToDB`
  (`/Game/Game/Components/AC_Database.SendEPDRadiationEventToDB` (`self.AC_Database`) :!label _label)
  (`KismetArrayLibrary.Array_Clear` (`self.CurrentEventDoseRateArray`))
  (`KismetArrayLibrary.Array_Clear` (`self.CurrentEventDoseAbsortionArray`))
  (`KismetArrayLibrary.Array_Clear` (`self.CurrentEventPositionArray`))
  (`KismetArrayLibrary.Array_Clear` (`self.CurrentEventDatetimeArray`)))

(event `self.SendLastEventsToDB`
  (`parent.SendLastEventsToDB`)
  (goto _label))

(fn `SetEPDId`
  (bind _outactors (`GameplayStatics.GetAllActorsOfClass` "BP_Dosimeter_EPD_C"))
  (if (`KismetArrayLibrary.Array_IsEmpty` _outactors)
    (set `self.EPDId` 0)
    (else
      (set `self.EPDId` (- (`KismetArrayLibrary.Array_Length` _outactors) 1)))))

(fn `UserConstructionScript`
  (`parent.UserConstructionScript`))