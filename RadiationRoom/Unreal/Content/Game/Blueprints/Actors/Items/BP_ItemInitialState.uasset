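; BP_ItemInitialState is a rotating display stand-in for an item, which SpawnItem swaps for the real pickable actor.
; On BeginPlay it looks up its item type in a data table, then shrinks and centers the mesh within its capsule, or destroys itself for the empty type.
; SpawnItem spawns the table's class for that type, destroys the stand-in and notifies BP_PlacePointManagers of matching type about the new BP_PickableItem.
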(event `self.ReceiveBeginPlay`
  (`MovementComponent.SetUpdatedComponent` (`self.RotatingMovement`) (`self.Item`))
  (if (`|EnumInequality` (`self.ItemType`) "NewEnumerator2")
    (`self.PutItemInByType` (`self.ItemType`))
    (else
      (`self.TakeItemOut`))))

(event `PutItemInByData`
  (params (ItemData :type "/Game/Game/DataStructures/Items/F_ItemData Structure"))
  (bind (_grouptype _type _id _name _description _image _mesh) (break `/Game/Game/DataStructures/Items/F_ItemData` ItemData))
  (set `self.ItemType` _type)
  (`StaticMeshComponent.SetStaticMesh` (`self.Item`) _mesh)
  (`self.SetItemScale`)
  (`self.SetItemLocation`))

(event `PutItemInByType`
  (params (ItemType :type "/Game/Game/DataStructures/Items/E_ItemType Enum" :default "NewEnumerator2"))
  (bind (_itemdata_grouptype _itemdata_type _itemdata_id _itemdata_name _itemdata_description _itemdata_image _itemdata_mesh) (break `/Game/Game/DataStructures/Items/F_ItemData` (`self.ItemData`)))
  (set `self.ItemType` ItemType)
  (`self.GetItemDataFromDataTable`)
  (`StaticMeshComponent.SetStaticMesh` (`self.Item`) _itemdata_mesh)
  (`self.SetItemScale`)
  (`self.SetItemLocation`))

(event `TakeItemOut`
  (set `self.ItemType` "NewEnumerator2")
  (`StaticMeshComponent.SetStaticMesh` (`self.Item`) null)
  (`self.K2_DestroyActor`))

(fn `AddSpawnedItemToPlacePointManagers`
  (params (Actor :type "/Game/Game/Blueprints/Actors/Items/BP_PickableItem Object Reference"))
  (bind _outactors (`GameplayStatics.GetAllActorsOfClass` "/Game/Game/Blueprints/Actors/Items/PlacePoints/BP_PlacePointManager.BP_PlacePointManager_C"))
  (for _array_element _outactors
    (if (`|EnumEquality` (`/Game/Game/Blueprints/Actors/Items/PlacePoints/BP_PlacePointManager.ItemType` _array_element) (`/Game/Game/Blueprints/Actors/Items/BP_InteractItemParent.ItemType` Actor))
      (`/Game/Game/Blueprints/Actors/Items/PlacePoints/BP_PlacePointManager.OnItemSpawned` _array_element Actor))))

(fn `GetItemClassFromDataTable`
  (returns (Class :type "Actor Class Reference"))
  (locals (CurrentItemClass :type "Actor Class Reference"))
  (bind _outrownames (`DataTableFunctionLibrary.GetDataTableRowNames` (`self.ItemData DataTable`)))
  (for _array_element _outrownames
    (bind _returnvalue (`|GetDataTableRow` (`self.ItemData DataTable`) _array_element)
      (:`then`
        (bind (_grouptype _type _id _name _description _image _mesh _class) (break `/Game/Game/DataStructures/Items/F_ItemData` _returnvalue))
        (if (`|EnumEquality` _type (`self.ItemType`))
          (set `local.CurrentItemClass` _class)))))
  (return (`local.CurrentItemClass`)))

(fn `GetItemDataFromDataTable`
  (bind _outrownames (`DataTableFunctionLibrary.GetDataTableRowNames` (`self.ItemData DataTable`)))
  (for _array_element _outrownames
    (bind _returnvalue (`|GetDataTableRow` (`self.ItemData DataTable`) _array_element)
      (:`then`
        (if (`|EnumEquality` (`.Type_32_18594ECA4CECEEEFD6D670A154F29F25` (break `/Game/Game/DataStructures/Items/F_ItemData` _returnvalue)) (`self.ItemType`))
          (set `self.ItemData` _returnvalue)
          (break))))))

(fn `GetItemId`
  (returns (`Item Data Id` :type "/Game/Game/DataStructures/Items/E_ItemType Enum"))
  (return "NewEnumerator2"))

(fn `GetMeshFromDataTable`
  (returns (` Mesh` :type "StaticMesh Object Reference"))
  (locals (CrrentItemMesh :type "StaticMesh Object Reference"))
  (bind _outrownames (`DataTableFunctionLibrary.GetDataTableRowNames` (`self.ItemData DataTable`)))
  (for _array_element _outrownames
    (bind _returnvalue (`|GetDataTableRow` (`self.ItemData DataTable`) _array_element)
      (:`then`
        (bind (_grouptype _type _id _name _description _image _mesh) (break `/Game/Game/DataStructures/Items/F_ItemData` _returnvalue))
        (if (`|EnumEquality` _type (`self.ItemType`))
          (set `local.CrrentItemMesh` _mesh)))))
  (return (`local.CrrentItemMesh`)))

(fn `SetItemLocation`
  (`SceneComponent.K2_SetWorldLocation` (`self.Item`) (- (`SceneComponent.K2_GetComponentLocation` (`self.Item`)) (- (`KismetSystemLibrary.GetComponentBounds` (`self.Item`)) (`KismetSystemLibrary.GetComponentBounds` (`self.Capsule`)))) false false))

(fn `SetItemScale`
  (bind _returnvalue (* (/ (`.SphereRadius` (`KismetSystemLibrary.GetComponentBounds` (`self.Capsule`))) (`.SphereRadius` (`KismetSystemLibrary.GetComponentBounds` (`self.Item`)))) 0.8))
  (`SceneComponent.SetWorldScale3D` (`self.Item`) (1.0 1.0 1.0))
  (if (< _returnvalue 1.0)
    (`SceneComponent.SetWorldScale3D` (`self.Item`) (* (`SceneComponent.K2_GetComponentScale` (`self.Item`)) _returnvalue))))

(fn `SpawnItem`
  (params (Transform :type "Transform Structure"))
  (returns (`Spawned Actor` :type "/Game/Game/Blueprints/Actors/Items/BP_PickableItem Object Reference"))
  (bind _class (`self.GetItemClassFromDataTable`))
  (bind _returnvalue (`|SpawnActorFromClass` _class Transform "Undefined" "MultiplyWithRoot" null null))
  (`self.TakeItemOut`)
  (bind _asbp_pickable_item (cast `/Game/Game/Blueprints/Actors/Items/BP_PickableItem` _returnvalue)
    (:`then`
      (`self.ED_ActorSpawned` _asbp_pickable_item)
      (`self.AddSpawnedItemToPlacePointManagers` _asbp_pickable_item)
      (return _asbp_pickable_item))
    (:`CastFailed`
      (return null))))

(fn `UserConstructionScript`)