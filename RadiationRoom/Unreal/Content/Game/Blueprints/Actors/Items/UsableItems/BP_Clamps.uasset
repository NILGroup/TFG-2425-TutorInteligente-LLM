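; BP_Clamps is a usable clamps item that picks up radiation emission point actors.
; When its sphere overlaps a BP_RadiationEmissionPoint, it stores that actor as the current item, links it back to itself and snaps it to the PointToGrab socket.
; Each pickup sends a timestamped interaction event, with user and scenario info from the game instance, to the database if that is valid.
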(event `self.ReceiveTick`
  (params (DeltaSeconds :type "Float (single-precision)"))
  (`parent.ReceiveTick` DeltaSeconds))

(event `self.Sphere.OnComponentBeginOverlap`
  (params (OverlappedComponent :type "PrimitiveComponent Object Reference") (OtherActor :type "Actor Object Reference") (OtherComp :type "PrimitiveComponent Object Reference") (OtherBodyIndex :type Integer) (bFromSweep :type Boolean) (SweepResult :type "HitResult Structure (by ref)"))
  (`self.SetItemInClamps` OtherActor))

(event `SetItemInClamps`
  (params (Actor :type "Actor Object Reference"))
  (bind _asbp_radiation_emission_point (cast `/Game/Game/Blueprints/Actors/Radiation/BP_RadiationEmissionPoint` Actor))
  (bind _output_get (set `self.CurrentItem` _asbp_radiation_emission_point))
  (set `/Game/Game/Blueprints/Actors/Radiation/BP_RadiationEmissionPoint.Clamps` self _output_get)
  (`self.K2_AttachToActor` _output_get self "PointToGrab" "SnapToTarget" "SnapToTarget" "KeepWorld" true)
  (set `self.HasItem` true)
  (`self.SendClampsInteractionEventToDB` "NewEnumerator1"))

(event `SendClampsInteractionEventToDB`
  (params (EvenType :type "/Game/Game/DataStructures/Database/E_ClampsInteractEventType Enum" :default "NewEnumerator0"))
  (bind _database_manager (`/Game/Game/FunctionLibraries/BFL_Common.GetMyDatabase`))
  (bind _data (`/Game/Game/Blueprints/RR_GameInstance.GetDataBaseMainInfoEvent` (`/Game/Game/FunctionLibraries/BFL_Common.GetMyGameInstance`)))
  (`/Engine/EditorBlueprintResources/StandardMacros.IsValid` _database_manager
    (:`Is Valid`
      (bind (_user_id _scenario_type) (break `/Game/Game/DataStructures/Database/F_MainInfoEvent` _data))
      (`/Game/Game/Blueprints/Database/BP_DataBase_Manager.SendClampsInteractionEventToDB` _database_manager (make `/Game/Game/DataStructures/Database/F_ClampsInteractionEvent` 0 _user_id _scenario_type EvenType (`KismetMathLibrary.Now`))))))

(fn `UserConstructionScript`
  (`parent.UserConstructionScript`))