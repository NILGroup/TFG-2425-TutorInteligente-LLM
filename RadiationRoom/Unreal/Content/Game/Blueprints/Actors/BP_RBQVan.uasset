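; BP_RBQVan is a van actor that spawns items requested through its child BP_RBQPanelActor.
; On the panel's spawn event, it sends the item IDs and quantities to the database through ACDatabase.
; It then spawns BP_ItemInitialState actors at random points just above its Plane's bounds, initialized from data table rows matched by type.
; It fires a dispatcher for each spawned item and one per item type.
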(event `self.ReceiveBeginPlay`
  (bind _asbp_rbqpanel_actor (cast `/Game/Game/Blueprints/Widgets/RBQPanels/BP_RBQPanelActor` (`ChildActorComponent.ChildActor` (`self.ChildActor`))))
  (add `/Game/Game/Blueprints/Widgets/RBQPanels/BP_RBQPanelActor.ED_SpawnItems` _asbp_rbqpanel_actor (delegate `SpawnItems`)))

(event `SpawnItems`
  (params (Items :type "Map of /Game/Game/DataStructures/Items/E_ItemType Enum to Integer"))
  (bind (_origin _boxextent) (`KismetSystemLibrary.GetComponentBounds` (`self.Plane`)))
  (`|ExecutionSequence`
    (:`then_0`
      (bind _keys (`BlueprintMapLibrary.Map_Keys` Items))
      (bind _listofids (`self.GetItemsIds` _keys))
      (bind _values (`BlueprintMapLibrary.Map_Values` Items))
      (`/Game/Game/Components/AC_Database.SendRBQEventToDB` (`self.AC_Database`) _listofids _values))
    (:`then_1`
      (bind _keys_2 (`BlueprintMapLibrary.Map_Keys` Items))
      (for _array_element _keys_2
        (bind _auxitemdata (`self.GetItemDataToSpawn` _array_element))
        (bind (_value _returnvalue) (`BlueprintMapLibrary.Map_Find` Items _array_element))
        (if _returnvalue
          (for _ (range _value)
            (bind _returnvalue_2 (`|SpawnActorFromClass` "/Game/Game/Blueprints/Actors/Items/BP_ItemInitialState.BP_ItemInitialState_C" (`KismetMathLibrary.MakeTransform` (+ (`KismetMathLibrary.RandomPointInBoundingBox` _origin _boxextent) (0.0 0.0 20.0))) "AdjustIfPossibleButAlwaysSpawn" "MultiplyWithRoot" null null))
            (`/Game/Game/Blueprints/Actors/Items/BP_ItemInitialState.PutItemInByData` _returnvalue_2 _auxitemdata)
            (`self.ED_ItemSpawned` _returnvalue_2))
          (`self.ED_MultipleItemsSpawned` _array_element _value))))))

(fn `GetItemDataToSpawn`
  (params (ItemType :type "/Game/Game/DataStructures/Items/E_ItemType Enum" :default "NewEnumerator2"))
  (returns (AuxItemData :type "/Game/Game/DataStructures/Items/F_ItemData Structure"))
  (bind _itemdata_datatable (`self.ItemData Datatable`))
  (bind _outrownames (`DataTableFunctionLibrary.GetDataTableRowNames` _itemdata_datatable))
  (for _array_element _outrownames
    (bind _returnvalue (`|GetDataTableRow` _itemdata_datatable _array_element)
      (:`then`
        (if (`|EnumEquality` (`.Type_32_18594ECA4CECEEEFD6D670A154F29F25` (break `/Game/Game/DataStructures/Items/F_ItemData` _returnvalue)) ItemType)
          (return _returnvalue))))))

(fn `GetItemsIds`
  (params (ItemTypes :type "Array of /Game/Game/DataStructures/Items/E_ItemType Enum"))
  (returns (ListOfIds :type "Array of Integer"))
  (locals (AuxList :type "Array of Integer"))
  (for _array_element ItemTypes
    (bind _auxitemdata (`self.GetItemDataToSpawn` _array_element))
    (`KismetArrayLibrary.Array_Add` (`local.AuxList`) (`.Id_31_2E96245D45DF11F5B0EEA7855F0A3C9C` (break `/Game/Game/DataStructures/Items/F_ItemData` _auxitemdata))))
  (return (`local.AuxList`)))

(fn `UserConstructionScript`)