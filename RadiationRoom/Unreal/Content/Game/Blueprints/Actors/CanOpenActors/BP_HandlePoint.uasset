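; BP_HandlePoint is a grabbable handle or knob point, filed with the openable actors, that reports when a player grabs or releases it.
; Its interact and cancel-interact events run the parent logic with the hand set to Left, then fire the OnKnobGrabStatusChanged dispatcher with true or false.
; It has no active logic of its own beyond these events, as BeginPlay, overlap and Tick are disabled.
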(event `/Game/Game/Interfaces/BI_ItemInteract.InteractWith`
  (params (Player :type "/Game/Game/Blueprints/Player/BP_Player Object Reference") (Hand :type "EControllerHand Enum" :default "Left"))
  (`parent.InteractWith` Player "Left")
  (`self.ED_OnKnobGrabStatusChanged` true))

(event `/Game/Game/Interfaces/BI_ItemInteract.CancelInteract`
  (params (Player :type "/Game/Game/Blueprints/Player/BP_Player Object Reference") (Hand :type "EControllerHand Enum" :default "Left"))
  (`parent.CancelInteract` Player "Left")
  (`self.ED_OnKnobGrabStatusChanged` false))

(fn `UserConstructionScript`
  (`parent.UserConstructionScript`))