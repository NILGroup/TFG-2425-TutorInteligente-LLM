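; Database manager actor that records gameplay telemetry such as user, interaction, movement, radiation, UI and tutorial events.
; On BeginPlay it spawns and binds BP_Database_LocalFile, and registers with the game instance after a short delay.
; Send events forward data to that backend's query builders; its closed and player-ID-found callbacks are re-broadcast through dispatchers.
; Shutdown broadcasts first, then closes the backend a second later; the timed query-flush logic is unwired.
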(event `self.ReceiveBeginPlay`
  (`|ExecutionSequence`
    (:`then_0`
      (`KismetSystemLibrary.Delay` 0.2)
      (`/Game/Game/Blueprints/RR_GameInstance.SetCurrentDataBase` (`/Game/Game/FunctionLibraries/BFL_Common.GetMyGameInstance`) self))
    (:`then_1`
      (bind _returnvalue (`|SpawnActorFromClass` "/Game/Game/Blueprints/Database/BP_Database_LocalFile.BP_Database_LocalFile_C" (`KismetMathLibrary.MakeTransform` (0.0 0.0 0.0)) "Undefined" "OverrideRootScale" null null))
      (set `self.LocalFileDB` _returnvalue)
      (`self.BindLocalFileDatabaseActions`))))

(event `self.ReceiveTick`
  (params (DeltaSeconds :type "Float (single-precision)")))

(event `BindLocalFileDatabaseActions`
  (bind _localfiledb (`self.LocalFileDB`))
  (add `/Game/Game/Blueprints/Database/BP_Database_LocalFile.ED_DatabaseClosed` _localfiledb (delegate `OnLocalFileDatabaseClosed`))
  (add `/Game/Game/Blueprints/Database/BP_Database_LocalFile.ED_PlayerIdFound` _localfiledb (delegate `OnPlayerIdFound`)))

(event `OnLocalFileDatabaseClosed`
  (set `self.LocalFileClosed` false)
  (`self.ED_DatabaseClosed`))

(event `OnPlayerIdFound`
  (params (Id :type Integer))
  (`self.ED_PlayerIdFound` Id))

(event `StopAndCloseDatabase`
  (`self.ED_DatabaseNeedToBeClosed`)
  (`KismetSystemLibrary.Delay` 1.0)
  (bind _localfiledb (`self.LocalFileDB`)
    (:`then`
      (`/Game/Game/Blueprints/Database/BP_Database_LocalFile.StopAndCloseDatabase` _localfiledb))
    (:`else`)))

(event `Get User Id`
  (params (`Player Name` :type String))
  (bind _localfiledb (`self.LocalFileDB`)
    (:`then`
      (`/Game/Game/Blueprints/Database/BP_Database_LocalFile.GetUserId` _localfiledb `Player Name`))
    (:`else`)))

(event `Send User to DB`
  (params (Data :type "/Game/Game/DataStructures/Database/F_User Structure"))
  (bind _localfiledb (`self.LocalFileDB`)
    (:`then`
      (`/Game/Game/Interfaces/BI_Database.CreateUserQuery` _localfiledb Data))
    (:`else`)))

(event `Send Item Interaction Event to DB`
  (params (Data :type "/Game/Game/DataStructures/Database/F_ItemInteractionEvent Structure"))
  (bind _localfiledb (`self.LocalFileDB`)
    (:`then`
      (`/Game/Game/Interfaces/BI_Database.CreateItemInteractionEventQuery` _localfiledb Data))
    (:`else`)))

(event `Send NPC Interaction Event to DB`
  (params (Data :type "/Game/Game/DataStructures/Database/F_NPCInteractionEvent Structure"))
  (bind _localfiledb (`self.LocalFileDB`)
    (:`then`
      (`/Game/Game/Interfaces/BI_Database.CreateNPCInteractionEventQuery` _localfiledb Data))
    (:`else`)))

(event `Send Gameplay Event to DB`
  (params (Data :type "/Game/Game/DataStructures/Database/F_GameplayEvent Structure"))
  (bind _localfiledb (`self.LocalFileDB`)
    (:`then`
      (`/Game/Game/Interfaces/BI_Database.CreateGameplayEventQuery` _localfiledb Data))
    (:`else`)))

(event `Send RBQ Event To DB`
  (params (Data :type "/Game/Game/DataStructures/Database/F_RBQEvent Structure"))
  (bind _localfiledb (`self.LocalFileDB`)
    (:`then`
      (`/Game/Game/Interfaces/BI_Database.CreateRBQEventQuery` _localfiledb Data))
    (:`else`)))

(event `Send Move Event to DB`
  (params (Data :type "/Game/Game/DataStructures/Database/F_MoveEvent Structure"))
  (bind _localfiledb (`self.LocalFileDB`)
    (:`then`
      (message `/Game/Game/Interfaces/BI_Database.CreateMoveEventQuery` _localfiledb Data))
    (:`else`)))

(event `Send Item Radiation Event To DB`
  (params (Data :type "/Game/Game/DataStructures/Database/F_ItemRadiationEvent Structure"))
  (bind _localfiledb (`self.LocalFileDB`)
    (:`then`
      (`/Game/Game/Interfaces/BI_Database.CreateItemRadiationEventQuery` _localfiledb Data))
    (:`else`)))

(event `Send PlacePoint Event to DB`
  (params (Data :type "/Game/Game/DataStructures/Database/F_PlacePointEvent Structure"))
  (bind _localfiledb (`self.LocalFileDB`)
    (:`then`
      (`/Game/Game/Interfaces/BI_Database.CreatePlacePointEventQuery` _localfiledb Data))
    (:`else`)))

(event `Send NPC Radiation Event To DB`
  (params (Data :type "/Game/Game/DataStructures/Database/F_NPCRadiationEvent Structure"))
  (bind _localfiledb (`self.LocalFileDB`)
    (:`then`
      (`/Game/Game/Interfaces/BI_Database.CreateNPCRadiationEventQuery` _localfiledb Data))
    (:`else`)))

(event `Send WalkieReport Event To DB`
  (params (Data :type "/Game/Game/DataStructures/Database/F_WalkieReportEvent Structure"))
  (bind _localfiledb (`self.LocalFileDB`)
    (:`then`
      (`/Game/Game/Interfaces/BI_Database.CreateWalkieReportEventQuery` _localfiledb Data))
    (:`else`)))

(event `Send EPD Radiation Event To DB`
  (params (Data :type "/Game/Game/DataStructures/Database/F_EPDRadiationEvent Structure"))
  (bind _localfiledb (`self.LocalFileDB`)
    (:`then`
      (`/Game/Game/Interfaces/BI_Database.CreateEPDRadiationEventQuery` _localfiledb Data))
    (:`else`)))

(event `Send User Radiation Event To DB`
  (params (Data :type "/Game/Game/DataStructures/Database/F_UserRadiationEvent Structure"))
  (bind _localfiledb (`self.LocalFileDB`)
    (:`then`
      (`/Game/Game/Interfaces/BI_Database.CreateUserRadiationEventQuery` _localfiledb Data))
    (:`else`)))

(event `Send Help Panel Event To DB`
  (params (Data :type "/Game/Game/DataStructures/Database/F_HelpPanelEvent Structure"))
  (bind _localfiledb (`self.LocalFileDB`)
    (:`then`
      (`/Game/Game/Interfaces/BI_Database.CreateHelpPanelEventQuery` _localfiledb Data))
    (:`else`)))

(event `Send Tips Event To DB`
  (params (Data :type "/Game/Game/DataStructures/Database/F_TipsEvent Structure"))
  (bind _localfiledb (`self.LocalFileDB`)
    (:`then`
      (`/Game/Game/Interfaces/BI_Database.CreateTipsEventQuery` _localfiledb Data))
    (:`else`)))

(event `SendClampsInteractionEventToDB`
  (params (Data :type "/Game/Game/DataStructures/Database/F_ClampsInteractionEvent Structure"))
  (bind _localfiledb (`self.LocalFileDB`)
    (:`then`
      (`/Game/Game/Interfaces/BI_Database.CreateClampsInteractionEventQuery` _localfiledb Data))
    (:`else`)))

(event `SendInventoryEventToDB`
  (params (Data :type "/Game/Game/DataStructures/Database/F_InventoryEvent Structure"))
  (bind _localfiledb (`self.LocalFileDB`)
    (:`then`
      (`/Game/Game/Interfaces/BI_Database.CreateInventoryEventQuery` _localfiledb Data))
    (:`else`)))

(event `SendUserInputEventToDB`
  (params (Data :type "/Game/Game/DataStructures/Database/F_UserInputEvent Structure"))
  (bind _localfiledb (`self.LocalFileDB`)
    (:`then`
      (`/Game/Game/Interfaces/BI_Database.CreateUserInputEventQuery` _localfiledb Data))
    (:`else`)))

(event `SendVideoEventToDB`
  (params (Data :type "/Game/Game/DataStructures/Database/F_VideoEvent Structure"))
  (bind _localfiledb (`self.LocalFileDB`)
    (:`then`
      (`/Game/Game/Interfaces/BI_Database.CreateVideoEventQuery` _localfiledb Data))
    (:`else`)))

(event `SendTutorialTaskEvent`
  (params (Data :type "/Game/Game/DataStructures/Database/F_TutorialTaskEvent Structure"))
  (bind _localfiledb (`self.LocalFileDB`)
    (:`then`
      (message `/Game/Game/Interfaces/BI_Database.CreateTutorialTaskEventQuery` _localfiledb Data))
    (:`else`)))

(fn `UserConstructionScript`)