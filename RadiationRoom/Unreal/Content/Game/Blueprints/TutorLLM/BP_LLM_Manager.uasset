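; Manager for Tuddy, an LLM-driven tutor buddy that the player toggles with T to type questions.
; StartLLM spawns the socket, message builder and buddy, creates the input panel, and connects to a local server.
; Init, sync and question messages go out as JSON with NPC dialog managers; init adds quest data and actor locations.
; Questions show a dotted "thinking" dialog; StopThinkingAndStartTuddyDialog only stops dialog, its start call being unwired.
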(event `EventConnectedToServer`
  (`self.ManageInitMessage`)
  (`KismetSystemLibrary.K2_SetTimerDelegate` (`|CreateDelegate` :!event `ManageSync`) 5.0 true)
  (`self.EnableInput` (`GameplayStatics.GetPlayerController` 0)))

(event `Key|T`
  (params (Key :type "Key Structure"))
  (:`Pressed`
    (if (`self.isInputDialogVisible`)
      (`self.HideInputDialog`)
      (`self.HideTuddy`)
      (else
        (`self.ShowAndMoveTuddy`)
        (if (not (`/Game/Game/Blueprints/TutorLLM/BP_TutorialBuddy_LLM.isInDialog` (`self.Tuddy`)))
          (`self.ShowInputDialog`))))))

(fn `HideInputDialog`
  (`Widget.RemoveFromParent` (`self.InputDialog`))
  (set `self.isInputDialogVisible` false))

(fn `HideTuddy`
  (`/Game/Game/Blueprints/Tutorial/BP_TutorialBuddy.Hide` (`self.Tuddy`)))

(fn `ManageInitMessage`
  (bind _jsoninitmsg (`/Game/Game/Blueprints/TutorLLM/BP_MessageBuilder.BuildInitMessage` (`self.MessageBuilder`) (`/Game/Game/Blueprints/Gameplay/BP_GameplayManager.Quest Data Table` (`/Game/Game/FunctionLibraries/BFL_Common.GetMyGameplayManager`)) (`BlueprintJsonLibrary.JsonMake`) (`self.NPCDialogManagers`) (`self.ElementsLocation`)))
  (`/Game/Game/Blueprints/TutorLLM/BP_Socket.Send Message` (`self.Socket`) (`BlueprintJsonLibrary.Conv_JsonObjectToString` _jsoninitmsg)))

(fn `ManageQuestion`
  (params (Text :type Text))
  (bind _jsonquestion (`/Game/Game/Blueprints/TutorLLM/BP_MessageBuilder.BuildQuestionMessage` (`self.MessageBuilder`) Text (`BlueprintJsonLibrary.JsonMake`) (`self.NPCDialogManagers`)))
  (`/Game/Game/Blueprints/TutorLLM/BP_Socket.Send Message` (`self.Socket`) (`BlueprintJsonLibrary.Conv_JsonObjectToString` _jsonquestion))
  (`self.HideInputDialog`)
  (`self.StartThinkingTuddy`))

(fn `ManageSync`
  (bind _jsonsync (`/Game/Game/Blueprints/TutorLLM/BP_MessageBuilder.BuildSyncMessage` (`self.MessageBuilder`) (`BlueprintJsonLibrary.JsonMake`) (`self.NPCDialogManagers`)))
  (`/Game/Game/Blueprints/TutorLLM/BP_Socket.Send Message` (`self.Socket`) (`BlueprintJsonLibrary.Conv_JsonObjectToString` _jsonsync)))

(fn `ShowAndMoveTuddy`
  (bind _returnvalue (`GameplayStatics.GetPlayerCharacter` 0))
  (`self.K2_SetActorLocationAndRotation` :`self` (`self.Tuddy`) :`NewLocation` (+ (`self.K2_GetActorLocation` _returnvalue) (* (`self.GetActorForwardVector` _returnvalue) (`KismetMathLibrary.Abs_Int` 200))) :`bTeleport` true)
  (`/Game/Game/Blueprints/Tutorial/BP_TutorialBuddy.Show` (`self.Tuddy`)))

(fn `ShowInputDialog`
  (`UserWidget.AddToViewport` (`self.InputDialog`) 0)
  (`WidgetBlueprintLibrary.SetInputMode_GameAndUIEx` (`GameplayStatics.GetPlayerController` 0) null)
  (set `self.isInputDialogVisible` true))

(fn `Start LLM`
  (`|ExecutionSequence`
    (:`then_0`
      (bind _returnvalue (`|CreateWidget` "/Game/Game/Blueprints/TutorLLM/WBP_TutorialBuddyInputPanel.WBP_TutorialBuddyInputPanel_C"))
      (set `self.InputDialog` _returnvalue)
      (bind _returnvalue_2 (`|SpawnActorFromClass` "/Game/Game/Blueprints/TutorLLM/BP_Socket.BP_Socket_C" (`KismetMathLibrary.MakeTransform` (0.0 0.0 0.0)) "Undefined" "MultiplyWithRoot" null null))
      (bind _output_get (set `self.Socket` _returnvalue_2))
      (set `/Game/Game/Blueprints/TutorLLM/BP_Socket.InputWidget` (`self.InputDialog`) _output_get)
      (bind _returnvalue_3 (`|SpawnActorFromClass` "/Game/Game/Blueprints/TutorLLM/BP_MessageBuilder.BP_MessageBuilder_C" (`KismetMathLibrary.MakeTransform` (0.0 0.0 0.0)) "Undefined" "MultiplyWithRoot" null null))
      (set `self.MessageBuilder` _returnvalue_3)
      (bind _returnvalue_4 (`|SpawnActorFromClass` "/Game/Game/Blueprints/TutorLLM/BP_TutorialBuddy_LLM.BP_TutorialBuddy_LLM_C" (`KismetMathLibrary.MakeTransform` (0.0 0.0 0.0)) "Undefined" "MultiplyWithRoot" null null))
      (set `self.Tuddy` _returnvalue_4)
      (bind _outactors (`GameplayStatics.GetAllActorsOfClass` "/Game/Game/Blueprints/Characters/BP_NPC_Talkable.BP_NPC_Talkable_C"))
      (for _array_element _outactors
        (`KismetArrayLibrary.Array_Add` (`self.NPCDialogManagers`) (`/Game/Game/Blueprints/Characters/BP_NPC_Talkable.AC_DialogManager` _array_element)))
      (bind _outactors_2 (`GameplayStatics.GetAllActorsOfClass` "/Script/Engine.Actor"))
      (for _array_element_2 _outactors_2
        (`BlueprintMapLibrary.Map_Add` (`self.ElementsLocation`) (`KismetSystemLibrary.GetObjectName` _array_element_2) (`self.K2_GetActorLocation` _array_element_2))))
    (:`then_1`
      (`WidgetBlueprintLibrary.SetInputMode_GameAndUIEx` (`GameplayStatics.GetPlayerController` 0) null)
      (set `self.isInputDialogVisible` false))
    (:`then_2`
      (add `/Game/Game/Blueprints/TutorLLM/WBP_TutorialBuddyInputPanel.onCommitedQuestion` (`self.InputDialog`) (`|CreateDelegate` :!event `ManageQuestion`))
      (add `/Game/Game/Blueprints/TutorLLM/BP_Socket.OnTutorFeedbackReceived` (`self.Socket`) (`|CreateDelegate` :!event `StartTuddyDialog`))
      (add `/Game/Game/Blueprints/TutorLLM/BP_Socket.OnConnectionStablished` (`self.Socket`) (`|CreateDelegate` :!event `EventConnectedToServer`)))
    (:`then_3`
      (`/Game/Game/Blueprints/TutorLLM/BP_Socket.StablishConnection` (`self.Socket`) "127.0.0.1" 65431))))

(fn `StartThinkingTuddy`
  (set `self.ThinkingTuddy` true)
  (`self.StartTuddyDialog` (`|MakeArray` "........................................" :!type "Text")))

(fn `StartTuddyDialog`
  (params (Message :type "Array of Text"))
  (bind _tuddy (`self.Tuddy`))
  (if (`self.ThinkingTuddy`)
    (set `self.ThinkingTuddy` false)
    (else
      (`self.ShowAndMoveTuddy`)))
  (set `/Game/Game/Blueprints/TutorLLM/BP_TutorialBuddy_LLM.isInDialog` true _tuddy)
  (`/Game/Game/Components/AC_TuddyDialogManager.StartNewDialog` (`/Game/Game/Blueprints/Tutorial/BP_TutorialBuddy.AC_TuddyDialogManager` _tuddy) "NewEnumerator0" Message))

(fn `StopThinkingAndStartTuddyDialog`
  (params (Dialog :type "Array of Text"))
  (`/Game/Game/Components/AC_TuddyDialogManager.StopDialog` (`/Game/Game/Blueprints/Tutorial/BP_TutorialBuddy.AC_TuddyDialogManager` (`self.Tuddy`))))

(fn `UserConstructionScript`)