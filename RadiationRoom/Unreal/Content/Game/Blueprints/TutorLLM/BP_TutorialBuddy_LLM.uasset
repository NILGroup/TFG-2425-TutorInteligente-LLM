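; LLM variant of the tutorial buddy actor, which in its current state mostly relies on inherited behavior.
; When the buddy's dialog completes, it clears the in-dialog flag and hides.
; Leftover, unconnected logic would bind a click event and open a tutorial buddy input panel with game-and-UI input.
; The click handler is empty, so no LLM interaction happens in this graph.
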(event `OnClicked_Event` :!signature `self.OnClicked`
  (params (TouchedActor :type "Actor Object Reference") (ButtonPressed :type "Key Structure" :default "None")))

(event `self.OnTuddyDialogCompleted`
  (params (CurrentTuddyDialogType :type "/Game/Game/DataStructures/Tutorial/E_TuddyDialogLinesType Enum" :default "NewEnumerator0") (CurrentExtraLineType :type "/Game/Game/DataStructures/Tutorial/E_TuddyExtraLineTypes Enum" :default "NewEnumerator1") (DialogID :type Name))
  (set `self.isInDialog` false)
  (`self.Hide`))

(fn `UserConstructionScript`
  (`parent.UserConstructionScript`))