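; TCP-style socket actor that links the game to the tutor LLM server, sending text as bytes and receiving tutor feedback.
; StablishConnection connects to a given IP and port, then a dispatcher fires once connected.
; Incoming 4-byte messages are read as integers, first the message count, then each string's length.
; Other messages are decoded into a text list, broadcast through OnTutorFeedbackReceived when the count runs out.
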(event `self.ReceiveBeginPlay`
  (set `self.MessageLength` 0)
  (set `self.MessagesRemaining` 0))

(event `onConnected`
  (params (ConnectionId :type Integer))
  (`self.OnConnectionStablished`))

(event `onDisconnected`
  (params (ConnectionId :type Integer)))

(event `onMessageReceived`
  (params (ConnectionId :type Integer) (Message :type "Array of Byte (by ref)"))
  (bind _returnvalue (== (`self.MessagesRemaining`) 0))
  (if (== (`KismetArrayLibrary.Array_Length` Message) 4)
    (bind _returnvalue_2 (`self.Message_ReadInt` Message))
    (if _returnvalue
      (set `self.MessagesRemaining` _returnvalue_2)
      (set `self.MessageList` (`|MakeArray`))
      (else
        (set `self.MessageLength` _returnvalue_2)))
    (else
      (bind _returnvalue_3 (`self.Message_ReadString` Message (`self.MessageLength`)))
      (`KismetArrayLibrary.Array_Add` (`self.MessageList`) (`KismetTextLibrary.Conv_StringToText` _returnvalue_3))
      (`/Engine/EditorBlueprintResources/StandardMacros.DecrementInt` (`self.MessagesRemaining`)
        (:`  `
          (if _returnvalue
            (`self.OnTutorFeedbackReceived` (`self.MessageList`))))))))

(fn `Send Message`
  (params (Text :type String))
  (`self.SendData` (`self.ServerConnectionId`) (`self.Conv_StringToBytes` Text)))

(fn `StablishConnection`
  (params (IP_Param :type String) (Port_Param :type Integer))
  (bind _output_get (set `self.IP` IP_Param))
  (bind _output_get_2 (set `self.Port` Port_Param))
  (bind _connectionid (`self.Connect` _output_get _output_get_2 (`|CreateDelegate` :!event `onDisconnected`) (`|CreateDelegate` :!event `onConnected`) (`|CreateDelegate` :!event `onMessageReceived`)))
  (set `self.ServerConnectionId` _connectionid))

(fn `UserConstructionScript`)