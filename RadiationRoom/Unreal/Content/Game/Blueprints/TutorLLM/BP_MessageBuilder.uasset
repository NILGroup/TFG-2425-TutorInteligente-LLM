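; Builds timestamped JSON messages of type init, sync and question that describe game state for the LLM tutor.
; Init gathers quest steps, level description, NPC dialog lines, element locations, player pose and tutorial text.
; Sync reports completed quests, each NPC's conversation state and player pose, and questions embed a fresh sync snapshot beside the text.
; Small Add functions each append one field to the JSON object passed through them.
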(fn `AddCurrentConversationData`
  (params (DialogManagers :type "Array of /Game/Game/Components/AC_NPCDialogManager Object Reference") (Json :type "BlueprintJsonObject Structure"))
  (returns (ConversationJson :type "BlueprintJsonObject Structure"))
  (locals (NPCs :type "Array of BlueprintJsonValue Structure"))
  (for _array_element DialogManagers
    (`KismetArrayLibrary.Array_Add` (`local.NPCs`) (`BlueprintJsonLibrary.JsonMakeObject` (`BlueprintJsonLibrary.JsonMakeField` (`BlueprintJsonLibrary.JsonMakeField` (`BlueprintJsonLibrary.JsonMakeField` (`BlueprintJsonLibrary.JsonMakeField` (`BlueprintJsonLibrary.JsonMake`) "name" (`BlueprintJsonLibrary.JsonMakeString` (`KismetSystemLibrary.GetObjectName` (`ActorComponent.GetOwner` _array_element)))) "conversation_index" (`BlueprintJsonLibrary.JsonMakeInt` (`/Game/Game/Components/AC_NPCDialogManager.ConversationIndex` _array_element))) "dialog_index" (`BlueprintJsonLibrary.JsonMakeInt` (`/Game/Game/Components/AC_NPCDialogManager.DialogIndex` _array_element))) "is_talking" (`BlueprintJsonLibrary.JsonMakeBool` (`/Game/Game/Components/AC_NPCDialogManager.IsTalking?` _array_element))))))
  (return (`BlueprintJsonLibrary.JsonMakeField` Json "npc_dialogs" (`BlueprintJsonLibrary.JsonMakeArray` (`local.NPCs`)))))

(fn `AddDescriptionLevelData`
  (params (Json :type "BlueprintJsonObject Structure"))
  (returns (JsonDescription :type "BlueprintJsonObject Structure"))
  (bind (_name _information) (break `/Game/Game/DataStructures/Scenarios/F_ScenarioDescription` (`/Game/Game/FunctionLibraries/BFL_Scenarios.GetCurrentScenarioDescription`)))
  (return (`BlueprintJsonLibrary.JsonMakeField` Json "level" (`BlueprintJsonLibrary.JsonMakeObject` (`BlueprintJsonLibrary.JsonMakeField` (`BlueprintJsonLibrary.JsonMakeField` (`BlueprintJsonLibrary.JsonMake`) "name" (`BlueprintJsonLibrary.JsonMakeString` (`KismetTextLibrary.Conv_TextToString` _name))) "description" (`BlueprintJsonLibrary.JsonMakeString` _information))))))

(fn `AddDialogData`
  (params (DialogManagers :type "Array of /Game/Game/Components/AC_NPCDialogManager Object Reference") (Json :type "BlueprintJsonObject Structure"))
  (returns (JsonDialogs :type "BlueprintJsonObject Structure"))
  (locals (Lines :type String) (Conversation :type "Array of BlueprintJsonValue Structure") (CharacterDialogs :type "Array of BlueprintJsonValue Structure"))
  (bind _lines (`local.Lines`))
  (for _array_element DialogManagers
    (for _array_element_2 (`/Game/Game/Components/AC_NPCDialogManager.Conversations` _array_element)
      (for _array_element_3 (`.DialogData_39_CA31413047BF35DEDAF362AFEAA84133` (break `/Game/Game/DataStructures/Dialogs/F_Conversation` _array_element_2))
        (if (`KismetStringLibrary.IsEmpty` _lines)
          (bind _returnvalue (`KismetTextLibrary.Conv_TextToString` (`.Text_2_8889C3EB4A46B35524B709947C974DCC` (break `/Game/Game/DataStructures/Dialogs/F_DialogLine` _array_element_3))))
          (set `local.Lines` _returnvalue)
          (else
            (set `local.Lines` (`KismetStringLibrary.Concat_StrStr` _lines "@" _returnvalue)))))
      (`KismetArrayLibrary.Array_Add` (`local.Conversation`) (`BlueprintJsonLibrary.JsonMakeString` (`local.Lines`)))
      (set `local.Lines` ""))
    (`KismetArrayLibrary.Array_Add` (`local.CharacterDialogs`) (`BlueprintJsonLibrary.JsonMakeObject` (`BlueprintJsonLibrary.JsonMakeField` (`BlueprintJsonLibrary.JsonMakeField` (`BlueprintJsonLibrary.JsonMake`) "name" (`BlueprintJsonLibrary.JsonMakeString` (`KismetSystemLibrary.GetObjectName` (`ActorComponent.GetOwner` _array_element)))) "dialog" (`BlueprintJsonLibrary.JsonMakeArray` (`local.Conversation`)))))
    (`KismetArrayLibrary.Array_Clear` (`local.Conversation`)))
  (return (`BlueprintJsonLibrary.JsonMakeField` Json "npc_dialogs" (`BlueprintJsonLibrary.JsonMakeArray` (`local.CharacterDialogs`)))))

(fn `AddElementsLocationData`
  (params (ElementsLocation :type "Map of String to Vector Structure") (Json :type "BlueprintJsonObject Structure"))
  (returns (`Json ElementsLocation` :type "BlueprintJsonObject Structure"))
  (locals (Items :type "Array of BlueprintJsonValue Structure"))
  (bind _keys (`BlueprintMapLibrary.Map_Keys` ElementsLocation))
  (for _array_element _keys
    (bind _json_position (`self.CoordsToJSON` (`BlueprintMapLibrary.Map_Find` ElementsLocation _array_element)))
    (`KismetArrayLibrary.Array_Add` (`local.Items`) (`BlueprintJsonLibrary.JsonMakeObject` (`BlueprintJsonLibrary.JsonMakeField` (`BlueprintJsonLibrary.JsonMakeField` (`BlueprintJsonLibrary.JsonMake`) "name" (`BlueprintJsonLibrary.JsonMakeString` _array_element)) "position" (`BlueprintJsonLibrary.JsonMakeObject` _json_position)))))
  (return (`BlueprintJsonLibrary.JsonMakeField` Json "elements_location" (`BlueprintJsonLibrary.JsonMakeArray` (`local.Items`)))))

(fn `AddPlayerLocationData`
  (params (Json :type "BlueprintJsonObject Structure"))
  (returns (`Json PlayerLocation` :type "BlueprintJsonObject Structure"))
  (bind _player (`/Game/Game/FunctionLibraries/BFL_Common.GetMyPlayer`))
  (bind _json_position (`self.CoordsToJSON` (`self.K2_GetActorLocation` _player)))
  (bind _json_position_2 (`self.CoordsToJSON` (`self.GetActorForwardVector` _player)))
  (return (`BlueprintJsonLibrary.JsonMakeField` Json "player" (`BlueprintJsonLibrary.JsonMakeObject` (`BlueprintJsonLibrary.JsonMakeField` (`BlueprintJsonLibrary.JsonMakeField` (`BlueprintJsonLibrary.JsonMake`) "position" (`BlueprintJsonLibrary.JsonMakeObject` _json_position)) "orientation" (`BlueprintJsonLibrary.JsonMakeObject` _json_position_2))))))

(fn `AddProgressData`
  (params (Json :type "BlueprintJsonObject Structure"))
  (returns (JsonProgress :type "BlueprintJsonObject Structure"))
  (locals (Quests :type "Array of BlueprintJsonValue Structure"))
  (bind _completedquests (`/Game/Game/Blueprints/Gameplay/BP_GameplayManager.CompletedQuests` (`/Game/Game/FunctionLibraries/BFL_Common.GetMyGameplayManager`)))
  (bind _keys (`BlueprintMapLibrary.Map_Keys` _completedquests))
  (for _array_element _keys
    (if (== (`BlueprintMapLibrary.Map_Find` _completedquests _array_element) true)
      (`KismetArrayLibrary.Array_Add` (`local.Quests`) (`BlueprintJsonLibrary.JsonMakeString` (`KismetStringLibrary.Conv_NameToString` _array_element)))))
  (return (`BlueprintJsonLibrary.JsonMakeField` Json "progress" (`BlueprintJsonLibrary.JsonMakeArray` (`local.Quests`)))))

(fn `AddStepsData`
  (params (StepsDT :type "DataTable Object Reference") (Json :type "BlueprintJsonObject Structure"))
  (returns (JsonSteps :type "BlueprintJsonObject Structure"))
  (locals (Quests :type "Array of BlueprintJsonValue Structure"))
  (bind _outrownames (`DataTableFunctionLibrary.GetDataTableRowNames` StepsDT))
  (for _array_element _outrownames
    (bind _returnvalue (`|GetDataTableRow` StepsDT _array_element)
      (:`then`
        (`KismetArrayLibrary.Array_Add` (`local.Quests`) (`BlueprintJsonLibrary.JsonMakeObject` (`BlueprintJsonLibrary.JsonMakeField` (`BlueprintJsonLibrary.JsonMakeField` (`BlueprintJsonLibrary.JsonMake`) "id" (`BlueprintJsonLibrary.JsonMakeString` (`KismetStringLibrary.Conv_NameToString` _array_element))) "description" (`BlueprintJsonLibrary.JsonMakeString` (`KismetTextLibrary.Conv_TextToString` (`.TrackingDescription_43_BB4922BA4D86CE9DBF3B05BA6612A06C` (break `/Game/Game/DataStructures/Gameplay/F_GameplayStepData` _returnvalue))))))))))
  (return (`BlueprintJsonLibrary.JsonMakeField` Json "steps" (`BlueprintJsonLibrary.JsonMakeArray` (`local.Quests`)))))

(fn `AddSyncData`
  (params (Json :type "BlueprintJsonObject Structure") (DialogManagers :type "Array of /Game/Game/Components/AC_NPCDialogManager Object Reference"))
  (returns (JsonData :type "BlueprintJsonObject Structure"))
  (bind _jsonprogress (`self.AddProgressData` (`BlueprintJsonLibrary.JsonMake`)))
  (bind _conversationjson (`self.AddCurrentConversationData` DialogManagers _jsonprogress))
  (bind _json_playerlocation (`self.AddPlayerLocationData` _conversationjson))
  (return (`BlueprintJsonLibrary.JsonMakeField` Json "data" (`BlueprintJsonLibrary.JsonMakeObject` _json_playerlocation))))

(fn `AddTimestamp`
  (params (Json :type "BlueprintJsonObject Structure"))
  (returns (JsonTimestamp :type "BlueprintJsonObject Structure"))
  (bind (_year _month _day _hour _minute _second _millisecond) (`KismetMathLibrary.BreakDateTime` (`KismetMathLibrary.Now`)))
  (return (`BlueprintJsonLibrary.JsonMakeField` Json "timestamp" (`BlueprintJsonLibrary.JsonMakeString` (`KismetStringLibrary.Replace` (`KismetTextLibrary.Conv_TextToString` (`|FormatText` "{Ano}/{Mes}/{Dia}_{Hora}:{Minuto}:{Segundo}.{Milisegundo}" (`KismetStringLibrary.Conv_IntToString` _year) _month _day _hour _minute _second _millisecond)) " ")))))

(fn `AddTutorialData`
  (params (Json :type "BlueprintJsonObject Structure"))
  (returns (JsonTutorial :type "BlueprintJsonObject Structure"))
  (locals (DT_Tutorial :type "DataTable Object Reference" :default "/Script/Engine.DataTable'/Game/Game/DataStructures/Tutorial/DT_TutorialItems_Quest.DT_TutorialItems_Quest'") (Instructions :type "Array of BlueprintJsonValue Structure"))
  (bind _outrownames (`DataTableFunctionLibrary.GetDataTableRowNames` (`local.DT_Tutorial`)))
  (for _array_element _outrownames
    (bind _returnvalue (`|GetDataTableRow` (`local.DT_Tutorial`) _array_element)
      (:`then`
        (bind (_type _id _title _description) (break `/Game/Game/DataStructures/Tutorial/F_TutorialItem` _returnvalue))
        (`KismetArrayLibrary.Array_Add` (`local.Instructions`) (`BlueprintJsonLibrary.JsonMakeObject` (`BlueprintJsonLibrary.JsonMakeField` (`BlueprintJsonLibrary.JsonMakeField` (`BlueprintJsonLibrary.JsonMake`) "title" (`BlueprintJsonLibrary.JsonMakeString` (`KismetTextLibrary.Conv_TextToString` _title))) "description" (`BlueprintJsonLibrary.JsonMakeString` (`KismetTextLibrary.Conv_TextToString` _description))))))))
  (return (`BlueprintJsonLibrary.JsonMakeField` Json "tutorial" (`BlueprintJsonLibrary.JsonMakeArray` (`local.Instructions`)))))

(fn `BuildInitMessage`
  (params (StepsDT :type "DataTable Object Reference") (Json :type "BlueprintJsonObject Structure") (`Dialog Managers` :type "Array of /Game/Game/Components/AC_NPCDialogManager Object Reference") (ElementsLocation :type "Map of String to Vector Structure"))
  (returns (JsonInitMsg :type "BlueprintJsonObject Structure"))
  (locals (Quests :type "Map of Name to Text"))
  (bind _jsonsteps (`self.AddStepsData` StepsDT (`BlueprintJsonLibrary.JsonMake`)))
  (bind _jsondescription (`self.AddDescriptionLevelData` _jsonsteps))
  (bind _jsondialogs (`self.AddDialogData` `Dialog Managers` _jsondescription))
  (bind _json_elementslocation (`self.AddElementsLocationData` ElementsLocation _jsondialogs))
  (bind _json_playerlocation (`self.AddPlayerLocationData` _json_elementslocation))
  (bind _jsontutorial (`self.AddTutorialData` _json_playerlocation))
  (bind _jsontimestamp (`self.AddTimestamp` (`BlueprintJsonLibrary.JsonMakeField` (`BlueprintJsonLibrary.JsonMakeField` Json "type" (`BlueprintJsonLibrary.JsonMakeString` "init")) "data" (`BlueprintJsonLibrary.JsonMakeObject` _jsontutorial))))
  (return _jsontimestamp))

(fn `BuildQuestionMessage`
  (params (Question :type Text) (Json :type "BlueprintJsonObject Structure") (DialogManagers :type "Array of /Game/Game/Components/AC_NPCDialogManager Object Reference"))
  (returns (JsonQuestion :type "BlueprintJsonObject Structure"))
  (bind _jsonsync (`self.BuildSyncMessage` (`BlueprintJsonLibrary.JsonMake`) DialogManagers))
  (bind _jsontimestamp (`self.AddTimestamp` (`BlueprintJsonLibrary.JsonMakeField` (`BlueprintJsonLibrary.JsonMakeField` (`BlueprintJsonLibrary.JsonMakeField` Json "type" (`BlueprintJsonLibrary.JsonMakeString` "question")) "text" (`BlueprintJsonLibrary.JsonMakeString` (`KismetTextLibrary.Conv_TextToString` Question))) "sync" (`BlueprintJsonLibrary.JsonMakeObject` _jsonsync))))
  (return _jsontimestamp))

(fn `BuildSyncMessage`
  (params (Json :type "BlueprintJsonObject Structure") (DialogManagers :type "Array of /Game/Game/Components/AC_NPCDialogManager Object Reference"))
  (returns (JsonSync :type "BlueprintJsonObject Structure"))
  (bind _jsondata (`self.AddSyncData` (`BlueprintJsonLibrary.JsonMakeField` Json "type" (`BlueprintJsonLibrary.JsonMakeString` "sync")) DialogManagers))
  (bind _jsontimestamp (`self.AddTimestamp` _jsondata))
  (return _jsontimestamp))

(fn `CoordsToJSON`
  (params (Position :type "Vector Structure"))
  (returns (`Json Position` :type "BlueprintJsonObject Structure"))
  (bind (_x _y _z) (`KismetMathLibrary.BreakVector3f` Position))
  (return (`BlueprintJsonLibrary.JsonMakeField` (`BlueprintJsonLibrary.JsonMakeField` (`BlueprintJsonLibrary.JsonMakeField` (`BlueprintJsonLibrary.JsonMake`) "X" (`BlueprintJsonLibrary.JsonMakeFloat` _x)) "Y" (`BlueprintJsonLibrary.JsonMakeFloat` _y)) "Z" (`BlueprintJsonLibrary.JsonMakeFloat` _z))))

(fn `UserConstructionScript`)