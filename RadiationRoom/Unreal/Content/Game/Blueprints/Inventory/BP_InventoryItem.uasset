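; BP_InventoryItem is an inventory slot that stores a pickable item and spawns it back out.
; A grabbed, acceptable item overlapping an empty slot's capsule turns it blue and binds its release event.
; Release with the inventory open stores the type, logs to the database and destroys the actor; take-out logs and clears the slot.
; EPD dosimeters regain their saved dose plus radiation the slot absorbed during storage when respawned.
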(event `self.Capsule.OnComponentBeginOverlap`
  (params (OverlappedComponent :type "PrimitiveComponent Object Reference") (OtherActor :type "Actor Object Reference") (OtherComp :type "PrimitiveComponent Object Reference") (OtherBodyIndex :type Integer) (bFromSweep :type Boolean) (SweepResult :type "HitResult Structure (by ref)"))
  (if (`|EnumEquality` (`self.ItemType`) "NewEnumerator2")
    (`/Engine/EditorBlueprintResources/StandardMacros.IsValid` OtherActor
      (:`Is Valid`
        (bind _asbp_pickable_item (cast `/Game/Game/Blueprints/Actors/Items/BP_PickableItem` OtherActor))
        (bind _can (`/Game/Game/Blueprints/Inventory/BP_Inventory.CanPutItemInto?` (`self.Inventory`) _asbp_pickable_item))
        (if _can
          (if (`/Game/Game/Blueprints/Actors/Items/BP_PickableItem.Grabbed` _asbp_pickable_item)
            (set `self.TargetItem` _asbp_pickable_item)
            (`self.BindTargetItemActions`)
            (`PrimitiveComponent.SetMaterial` (`self.Capsule`) 0 "/Game/Game/Assets/Materials/TranslucentBasicColors/M_Blue.M_Blue")))))))

(event `self.Capsule.OnComponentEndOverlap`
  (params (OverlappedComponent :type "PrimitiveComponent Object Reference") (OtherActor :type "Actor Object Reference") (OtherComp :type "PrimitiveComponent Object Reference") (OtherBodyIndex :type Integer))
  (if (`|EnumEquality` (`self.ItemType`) "NewEnumerator2")
    (`/Engine/EditorBlueprintResources/StandardMacros.IsValid` OtherActor
      (:`Is Valid`
        (if (== OtherActor (`self.TargetItem`))
          (remove `/Game/Game/Blueprints/Actors/Items/BP_InteractItemParent.ED_InteractionCompleted` (`self.TargetItem`) (delegate `OnTargetItemRelease`))
          (set `self.TargetItem` null)
          (`PrimitiveComponent.SetMaterial` (`self.Capsule`) 0 "/Game/Game/Assets/Materials/TranslucentBasicColors/M_Translucent.M_Translucent"))))))

(event `self.TakeItemOut`
  (bind (_itemdata_grouptype _itemdata_type _itemdata_id) (break `/Game/Game/DataStructures/Items/F_ItemData` (`self.ItemData`)))
  (if (`|EnumInequality` (`self.ItemType`) "NewEnumerator2")
    (`/Game/Game/Blueprints/Inventory/BP_Inventory.SendInventoryEventToDB` (`self.Inventory`) _itemdata_id "NewEnumerator2" (`|GetEnumeratorNameAsString` _itemdata_type))
    (set `self.ItemType` "NewEnumerator2")
    (`StaticMeshComponent.SetStaticMesh` (`self.Item`) null)))

(event `SaveItemSpecialFeatures`
  (params (Actor :type "/Game/Game/Blueprints/Actors/Items/BP_PickableItem Object Reference"))
  (switch `/Game/Game/DataStructures/Items/E_ItemType` (`/Game/Game/Blueprints/Actors/Items/BP_InteractItemParent.ItemType` Actor)
    (:`NewEnumerator3`
      (bind _asbp_dosimeter_epd (cast `/Game/Game/Blueprints/Actors/Dosimeters/BP_Dosimeter_EPD` Actor))
      (set `self.EPD Absortion Dose` (`/Game/Game/Components/AC_Radiation.DoseAbsorption` (`/Game/Game/Blueprints/Actors/Items/BP_InteractItemParent.AC_Radiation` _asbp_dosimeter_epd)))
      (set `/Game/Game/Components/AC_Radiation.DoseAbsorption` 0.0 (`self.AC_Radiation`)))))

(event `BindTargetItemActions`
  (bind _targetitem (`self.TargetItem`)
    (:`then`
      (add `/Game/Game/Blueprints/Actors/Items/BP_InteractItemParent.ED_InteractionCompleted` _targetitem (delegate `OnTargetItemRelease`)))
    (:`else`)))

(event `OnTargetItemRelease`
  (params (Actor :type "/Game/Game/Blueprints/Actors/Items/BP_InteractItemParent Object Reference"))
  (bind _targetitem (`self.TargetItem`))
  (if (`/Game/Game/Blueprints/Inventory/BP_Inventory.IsOpen` (`self.Inventory`))
    (`self.PutItemInByType` (`/Game/Game/Blueprints/Actors/Items/BP_InteractItemParent.ItemType` _targetitem))
    (`self.SaveItemSpecialFeatures` _targetitem)
    (`/Game/Game/Blueprints/Inventory/BP_Inventory.SendInventoryEventToDB` (`self.Inventory`) (`/Game/Game/Blueprints/Actors/Items/BP_InteractItemParent.ActorId` _targetitem) "NewEnumerator1" (`KismetSystemLibrary.GetDisplayName` _targetitem))
    (`self.K2_DestroyActor` _targetitem)
    (`PrimitiveComponent.SetMaterial` (`self.Capsule`) 0 "/Game/Game/Assets/Materials/TranslucentBasicColors/M_Translucent.M_Translucent")))

(fn `SpawnItem`
  (params (Transform :type "Transform Structure"))
  (returns (`Spawned Actor` :type "/Game/Game/Blueprints/Actors/Items/BP_PickableItem Object Reference"))
  (bind _yes (`/Game/Game/Blueprints/Inventory/BP_Inventory.CanTakeOut?` (`self.Inventory`)))
  (if _yes
    (bind _spawned_actor (`parent.SpawnItem` Transform))
    (bind _asbp_dosimeter_epd (cast `/Game/Game/Blueprints/Actors/Dosimeters/BP_Dosimeter_EPD` _spawned_actor)
      (:`then`
        (set `/Game/Game/Components/AC_Radiation.DoseAbsorption` (+ (`self.EPD Absortion Dose`) (`/Game/Game/Components/AC_Radiation.DoseAbsorption` (`self.AC_Radiation`))) (`/Game/Game/Blueprints/Actors/Items/BP_InteractItemParent.AC_Radiation` _asbp_dosimeter_epd)))
      (:`CastFailed`
        _))
    (return _spawned_actor)
    (else
      (return null))))

(fn `UserConstructionScript`)