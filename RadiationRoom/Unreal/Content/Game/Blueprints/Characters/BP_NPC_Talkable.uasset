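; BP_NPC_Talkable is an NPC that the player can talk to inside a talk area.
; Entering the area while talking is allowed shows a start-talking widget button and enables looking at the player; leaving hides it and stops the conversation.
; Pressing the button calls InteractWith, with dialogue handled by ACDialogManager using a typewriter text component.
; Finished conversations are re-broadcast through the NPC's own event dispatcher.
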(event `self.ReceiveBeginPlay`
  (`parent.ReceiveBeginPlay`)
  (set `self.CanLookPlayer` false)
  (`self.InitStartTalkingButton`)
  (add `/Game/Game/Components/AC_NPCDialogManager.ConversationFinished` (`self.AC_DialogManager`) (delegate `EventDispachedConversationFinished`))
  (`/Game/Game/Components/AC_NPCDialogManager.SetTypewriterComponent` (`self.AC_DialogManager`) (`self.AC_TypewriterText`)))

(event `EventDispachedConversationFinished`
  (params (`Conversation Number` :type Integer))
  (`self.Conversation Finished` `Conversation Number`))

(event `self.ReceiveTick`
  (params (DeltaSeconds :type "Float (single-precision)"))
  (`parent.ReceiveTick` DeltaSeconds))

(event `PlayerIsAlreadyOverlapping`
  ;[1 1 1] Talk Area
  (if (`PrimitiveComponent.IsOverlappingActor` (`self.TalkArea`) (`/Game/Game/FunctionLibraries/BFL_Common.GetMyPlayer`))
    (if (and (`self.CanTalk`) (not (`/Game/Game/Components/AC_NPCDialogManager.IsTalking?` (`self.AC_DialogManager`)))) :!label _label
      (set `self.CanLookPlayer` true)
      (`SceneComponent.SetHiddenInGame` (`self.StartTalkingButtonWidgetComponent`) false false))))

(event `self.TalkArea.OnComponentBeginOverlap`
  (params (OverlappedComponent :type "PrimitiveComponent Object Reference") (OtherActor :type "Actor Object Reference") (OtherComp :type "PrimitiveComponent Object Reference") (OtherBodyIndex :type Integer) (bFromSweep :type Boolean) (SweepResult :type "HitResult Structure (by ref)"))
  ;[1 1 1] Talk Area
  (if (== OtherActor (`/Game/Game/FunctionLibraries/BFL_Common.GetMyPlayer`))
    (goto _label)))

(event `self.TalkArea.OnComponentEndOverlap`
  (params (OverlappedComponent :type "PrimitiveComponent Object Reference") (OtherActor :type "Actor Object Reference") (OtherComp :type "PrimitiveComponent Object Reference") (OtherBodyIndex :type Integer))
  ;[1 1 1] Talk Area
  (if (== OtherActor (`/Game/Game/FunctionLibraries/BFL_Common.GetMyPlayer`))
    (set `self.CanLookPlayer` false)
    (`/Game/Game/Components/AC_NPCDialogManager.StopConversation` (`self.AC_DialogManager`))
    (`SceneComponent.SetHiddenInGame` (`self.StartTalkingButtonWidgetComponent`) true false)))

(event `/Game/Game/Interfaces/BI_NPCInteract.InteractWith`
  (params (Player :type "/Game/Game/Blueprints/Player/BP_Player Object Reference"))
  ;[1 1 1] Interact
  (`parent.InteractWith` Player)
  (`/Game/Game/Components/AC_NPCDialogManager.Interact With` (`self.AC_DialogManager`)))

(event `/Game/Game/Interfaces/BI_NPCInteract.CancelInteract`
  (params (Player :type "/Game/Game/Blueprints/Player/BP_Player Object Reference"))
  ;[1 1 1] Interact
  (`parent.CancelInteract` Player))

(event `NextConversation`
  (`/Game/Game/Components/AC_NPCDialogManager.NextConversation` (`self.AC_DialogManager`)))

(event `Conversation Finished`
  (params (`Conversation Number` :type Integer))
  (`self.ED_ConversationFinished` `Conversation Number`))

(event `InitStartTalkingButton`
  (`SceneComponent.SetHiddenInGame` (`self.StartTalkingButtonWidgetComponent`) true false)
  (`SceneComponent.SetHiddenInGame` (`self.DialogWidgetComponent`) true false)
  (bind _aswbp_start_talking_button (cast `/Game/Game/UserInterfaces/Dialogs/WBP_StartTalkingButton` (`WidgetComponent.GetWidget` (`self.StartTalkingButtonWidgetComponent`))))
  (bind _output_get (set `self.StartTalkingWidgetActor` _aswbp_start_talking_button))
  (add `/Game/Game/UserInterfaces/Dialogs/WBP_StartTalkingButton.ED_StartTalking` _output_get (delegate `OnStartTalkingButtonPressed`)))

(event `OnStartTalkingButtonPressed`
  (`/Game/Game/Interfaces/BI_NPCInteract.InteractWith` (`/Game/Game/Blueprints/RR_GameInstance.CurrentPlayer` (`self.GameInstance`)))
  (`SceneComponent.SetHiddenInGame` (`self.StartTalkingButtonWidgetComponent`) true false))

(fn `UserConstructionScript`)