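; Gameplay manager for the second tutorial scenario, running a radiation-response quest chain (T2001–T2005) framed by guide dialogs and countdown widgets.
; It extends parent events and binds delegates on van-spawned and placed items, the tutorial manager and triggers.
; Van spawns, walkie-talkie report, dosimeter readings and a tutorial menu selection successively complete quests.
; Once gameplay is completed, the end trigger starts the closing dialog and countdown before ending play.
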(event `self.CheatButton`
  ;[1 1 1] Cheat Button
  (`parent.CheatButton`)
  (`self.CompleteQuest` (`|GetArrayItem` (`self.SortedQuests`) (`self.CurrentQuestIndex`)))
  (if (< (`self.CurrentQuestIndex`) (- (`KismetArrayLibrary.Array_Length` (`self.SortedQuests`)) 1))
    (bind _result (`/Engine/EditorBlueprintResources/StandardMacros.IncrementInt` (`self.CurrentQuestIndex`))
      (:`  `
        (`self.SetCurrentQuest` (`|GetArrayItem` (`self.SortedQuests`) _result))))))

(event `self.ReceiveBeginPlay`
  (`parent.ReceiveBeginPlay`)
  (`|ExecutionSequence`
    (:`then_0`
      (set `self.CanStartCurrentQuest` false))
    (:`then_1`
      (`self.SetActorHiddenInGame` (`self.GoodbyeWidget`) true))
    (:`then_2`
      (bind _tutorialmanager (`self.TutorialManager`)
        (:`then`
          (set `/Game/Game/Blueprints/Tutorial/BP_TutorialManager.PlayerCanDemandTuddy` false _tutorialmanager)
          (`self.BindTutorialManagerActions`))
        (:`else`
          (`/Game/Game/Blueprints/RR_GameInstance.Log` (`/Game/Game/FunctionLibraries/BFL_Common.GetMyGameInstance`) "NewEnumerator2" "Falta el TutorialManager" false))))))

(event `self.StartScenario`
  (bind _starttuddy (`self.StartTuddy`))
  (`parent.StartScenario`)
  (`/Game/Game/Blueprints/Tutorial/BP_TutorialBuddy.Show` _starttuddy)
  (`KismetSystemLibrary.Delay` 0.5)
  (`/Game/Game/Components/AC_TuddyDialogManager.StartNewDialogByID` (`/Game/Game/Blueprints/Tutorial/BP_TutorialBuddy.AC_TuddyDialogManager` _starttuddy) "T2001"))

(event `self.CompleteQuest`
  (params (QuestID :type Name))
  (`parent.CompleteQuest` QuestID)
  (`/Game/Game/Blueprints/Tutorial/BP_TutorialDisplayManager.NextDisplay` (`self.TutorialDisplayManager`))
  (if (`self.GameplayCompleted`)
    (`KismetSystemLibrary.Delay` 1.0)
    (`/Game/Game/Blueprints/Tutorial/BP_TutorialBuddy.Show` (`self.EndTuddy`))
    (`self.SetActorHiddenInGame` (`self.GoodbyeWidget`) false)))

(event `self.OnGameInstancePlayerSetted`
  (`parent.OnGameInstancePlayerSetted`)
  (`/Game/Game/Blueprints/Tutorial/BP_TutorialManager.SetCurrentTutorialBuddy` (`self.TutorialManager`) (`/Game/Game/Blueprints/Player/BP_Player_VR.TutorialBuddyActor` (`/Game/Game/FunctionLibraries/BFL_Common.GetMyPlayer`)))
  (`self.BindTuddyActions`))

(event `self.BindTuddyActions`
  (`parent.BindTuddyActions`)
  (add `/Game/Game/Components/AC_TuddyDialogManager.ED_DialogCompleted` (`/Game/Game/Blueprints/Tutorial/BP_TutorialBuddy.AC_TuddyDialogManager` (`self.StartTuddy`)) (delegate `OnStartTuddyDialogCompleted`))
  (add `/Game/Game/Components/AC_TuddyDialogManager.ED_DialogCompleted` (`/Game/Game/Blueprints/Tutorial/BP_TutorialBuddy.AC_TuddyDialogManager` (`self.EndTuddy`)) (delegate `OnEndTuddyDialogCompleted`)))

(event `OnStartTuddyDialogCompleted`
  (params (CurrentTuddyDialogType :type "/Game/Game/DataStructures/Tutorial/E_TuddyDialogLinesType Enum" :default "NewEnumerator0") (CurrentExtraLineType :type "/Game/Game/DataStructures/Tutorial/E_TuddyExtraLineTypes Enum" :default "NewEnumerator1") (DialogID :type Name))
  (bind _welcomewidget (`self.WelcomeWidget`))
  (`/Game/Game/Blueprints/Tutorial/BP_TutorialBuddy.Hide` (`self.StartTuddy`))
  (`self.SetActorHiddenInGame` (`self.WelcomeWidget`) false)
  (`/Game/Game/Blueprints/Tutorial/BP_PanelWithCountdown.StartCountdown` _welcomewidget)
  (add `/Game/Game/Blueprints/Tutorial/BP_PanelWithCountdown.ED_CountdownEnded` _welcomewidget (delegate `OnWelcomeCountdownCompleted`)))

(event `OnWelcomeCountdownCompleted`
  (`self.K2_SetActorLocation` (`/Game/Game/FunctionLibraries/BFL_Common.GetMyPlayer`) (`self.K2_GetActorLocation` (`self.InitialTeleportPoint`)) false true)
  (`self.SetCurrentQuest` "T2001")
  (`/Game/Game/Blueprints/Tutorial/BP_TutorialDisplayManager.StartFirstDisplay` (`self.TutorialDisplayManager`)))

(event `OnEndTuddyDialogCompleted`
  (params (CurrentTuddyDialogType :type "/Game/Game/DataStructures/Tutorial/E_TuddyDialogLinesType Enum" :default "NewEnumerator0") (CurrentExtraLineType :type "/Game/Game/DataStructures/Tutorial/E_TuddyExtraLineTypes Enum" :default "NewEnumerator1") (DialogID :type Name))
  (bind _goodbyewidget (`self.GoodbyeWidget`))
  (`/Game/Game/Blueprints/Tutorial/BP_TutorialBuddy.Hide` (`self.EndTuddy`))
  (`self.SetActorHiddenInGame` (`self.GoodbyeWidget`) false)
  (`/Game/Game/Blueprints/Tutorial/BP_PanelWithCountdown.StartCountdown` _goodbyewidget)
  (add `/Game/Game/Blueprints/Tutorial/BP_PanelWithCountdown.ED_CountdownEnded` _goodbyewidget (delegate `OnGoodbyeCountdownCompleted`)))

(event `OnGoodbyeCountdownCompleted`
  (`self.EndGameplay`))

(event `BindTutorialManagerActions`
  (add `/Game/Game/Blueprints/Tutorial/BP_TutorialManager.ED_TutorialDemandedItemSelected` (`self.TutorialManager`) (delegate `OnTutorialItemSelected`)))

(event `OnTutorialItemSelected`
  (params (`Tutorial Item ID` :type "/Game/Game/DataStructures/Tutorial/E_TutorialItemID Enum" :default "NewEnumerator0"))
  (if (`self.Is Current Quest and Can Start` "T2005")
    (switch `/Game/Game/DataStructures/Tutorial/E_TutorialItemID` `Tutorial Item ID`
      (:`NewEnumerator3`
        (`KismetSystemLibrary.Delay` 1.0)
        (`self.CompleteQuest` (`self.CurrentQuestID`))))))

(event `self.BindPlayerActions`
  (`parent.BindPlayerActions`)
  (add `self.OnActorBeginOverlap` (`self.EndTrigger`) (delegate `OnActorOverlapEndTrigger`)))

(event `OnActorOverlapEndTrigger` :!signature `self.OnActorBeginOverlap`
  (params (OverlappedActor :type "Actor Object Reference") (OtherActor :type "Actor Object Reference"))
  (if (== OtherActor (`/Game/Game/FunctionLibraries/BFL_Common.GetMyPlayer`))
    (if (`self.GameplayCompleted`)
      (`/Game/Game/Components/AC_TuddyDialogManager.StartNewDialogByID` (`/Game/Game/Blueprints/Tutorial/BP_TutorialBuddy.AC_TuddyDialogManager` (`self.EndTuddy`)) "T2002"))))

(event `self.BindItemActions`
  (`parent.BindItemActions`)
  (`|ExecutionSequence`
    (:`then_0`
      (`self.BindRBQVanEvents`))
    (:`then_1`
      (bind _returnvalue (`GameplayStatics.GetActorOfClass` "/Game/Game/Blueprints/WalkieTalkie/BP_WalkieTalkie.BP_WalkieTalkie_C"))
      (bind _output_get (set `self.Walkie-Talkie` _returnvalue))
      (`self.BindWalkieTalkieEvents` _output_get))
    (:`then_2`
      (bind _outactors (`GameplayStatics.GetAllActorsOfClass` "/Game/Game/Blueprints/Actors/Dosimeters/BP_Dosimeter_SABG100.BP_Dosimeter_SABG100_C"))
      (for _array_element _outactors
        (`self.BindSAGB100Actions` _array_element)))
    (:`then_3`
      (bind _outactors_2 (`GameplayStatics.GetAllActorsOfClass` "/Game/Game/Blueprints/Actors/Dosimeters/BP_Dosimeter_EPD.BP_Dosimeter_EPD_C"))
      (for _array_element_2 _outactors_2
        (`self.BindEPDActions` _array_element_2)))))

(event `BindRBQVanEvents`
  (bind _returnvalue (`GameplayStatics.GetActorOfClass` "/Game/Game/Blueprints/Actors/BP_RBQVan.BP_RBQVan_C"))
  (set `self.RBQVan` _returnvalue)
  (bind _rbqvan (`self.RBQVan`)
    (:`then`
      (add `/Game/Game/Blueprints/Actors/BP_RBQVan.ED_ItemSpawned` _rbqvan (delegate `OnRBQItemSpawned`)))
    (:`else`
      (`/Game/Game/Blueprints/RR_GameInstance.Log` (`/Game/Game/FunctionLibraries/BFL_Common.GetMyGameInstance`) "NewEnumerator2" "Falta RBQ Van" false))))

(event `OnRBQItemSpawned`
  (params (Actor :type "/Game/Game/Blueprints/Actors/Items/BP_ItemInitialState Object Reference"))
  (if (`self.Is Current Quest and Can Start` "T2001")
    (`|ExecutionSequence`
      (:`then_0`
        (switch `/Game/Game/DataStructures/Items/E_ItemType` (`/Game/Game/Blueprints/Actors/Items/BP_ItemInitialState.ItemType` Actor)
          (:`NewEnumerator0`
            (bind _result (`/Engine/EditorBlueprintResources/StandardMacros.IncrementInt` (`self.NumOfTrafficConesSpawned`))
              (:`  `
                (set `self.NumOfTrafficConesSpawned` _result))))
          (:`NewEnumerator1`
            (bind _result_2 (`/Engine/EditorBlueprintResources/StandardMacros.IncrementInt` (`self.NumOfSABG100Spawned`))
              (:`  `
                (set `self.NumOfSABG100Spawned` _result_2))))))
      (:`then_1`
        (if (and (>= (`self.NumOfTrafficConesSpawned`) 2) (>= (`self.NumOfSABG100Spawned`) 1))
          (`self.CompleteQuest` (`self.CurrentQuestID`))
          (`self.SetCurrentQuest` "T2002")))
      (:`then_2`
        (add `/Game/Game/Blueprints/Actors/Items/BP_ItemInitialState.ED_ActorSpawned` Actor (delegate `OnRBQActorSpawned`))))))

(event `OnRBQActorSpawned`
  (params (Actor :type "/Game/Game/Blueprints/Actors/Items/BP_PickableItem Object Reference"))
  (bind _asbp_walkie_talkie (cast `/Game/Game/Blueprints/WalkieTalkie/BP_WalkieTalkie` Actor)
    (:`then`
      (`self.BindWalkieTalkieEvents` _asbp_walkie_talkie))
    (:`CastFailed`
      (bind _asbp_dosimeter_sabg100 (cast `/Game/Game/Blueprints/Actors/Dosimeters/BP_Dosimeter_SABG100` Actor)
        (:`then`
          (`self.BindSAGB100Actions` _asbp_dosimeter_sabg100))
        (:`CastFailed`
          (bind _asbp_dosimeter_epd (cast `/Game/Game/Blueprints/Actors/Dosimeters/BP_Dosimeter_EPD` Actor))
          (`self.BindEPDActions` _asbp_dosimeter_epd))))))

(event `BindWalkieTalkieEvents`
  (params (WalkieTalkie :type "/Game/Game/Blueprints/WalkieTalkie/BP_WalkieTalkie Object Reference"))
  (set `/Game/Game/Blueprints/WalkieTalkie/BP_WalkieTalkie.CanShowDialogBox` false WalkieTalkie)
  (add `/Game/Game/Blueprints/WalkieTalkie/BP_WalkieTalkie.ED_InitialReportCompleted` WalkieTalkie (delegate `OnWalkieInitialReportCompleted`)))

(event `OnWalkieInitialReportCompleted`
  (if (`self.Is Current Quest and Can Start` "T2002")
    (`self.CompleteQuest` (`self.CurrentQuestID`))
    (`self.SetCurrentQuest` "T2003")))

(event `BindSAGB100Actions`
  (params (SABG100 :type "/Game/Game/Blueprints/Actors/Dosimeters/BP_Dosimeter_SABG100 Object Reference"))
  (add `/Game/Game/Blueprints/Actors/Dosimeters/BP_Dosimeter_SABG100.ED_ItemRadiationMeasured` SABG100 (delegate `OnSABG100ItemRadiationMeasured`))
  (add `/Game/Game/Blueprints/Actors/Dosimeters/BP_Dosimeter_SABG100.ED_NPCRadiationMeasured` SABG100 (delegate `ONSABG100NPCRadiationMeasured`)))

(event `OnSABG100ItemRadiationMeasured`
  (params (Actor :type "/Game/Game/Blueprints/Actors/Items/BP_InteractItemParent Object Reference"))
  (if (`self.CanUseSABG100`)
    (if (`self.Is Current Quest and Can Start` "T2003")
      (bind _output_get (set `self.Item Radiation Measured` true))
      (if (and _output_get (`self.NPCRadiation Measured`))
        (`self.CompleteQuest` (`self.CurrentQuestID`) :!label _label)
        (`self.SetCurrentQuest` "T2004")))))

(event `ONSABG100NPCRadiationMeasured`
  (params (Actor :type "/Game/Game/Blueprints/Characters/BP_NPC Object Reference"))
  (if (`self.CanUseSABG100`)
    (if (`self.Is Current Quest` "T2003")
      (bind _output_get (set `self.NPCRadiation Measured` true))
      (if (and _output_get (`self.Item Radiation Measured`))
        (goto _label)))))

(event `BindEPDActions`
  (params (EPD :type "/Game/Game/Blueprints/Actors/Dosimeters/BP_Dosimeter_EPD Object Reference"))
  (add `self.OnActorBeginOverlap` (`self.RadiationEmissionPointSphereTrigger`) (delegate `OnEPDOverlapped`)))

(event `OnEPDOverlapped` :!signature `self.OnActorBeginOverlap`
  (params (OverlappedActor :type "Actor Object Reference") (OtherActor :type "Actor Object Reference"))
  (if (`self.CanUseEPD`)
    (bind _asbp_dosimeter_epd (cast `/Game/Game/Blueprints/Actors/Dosimeters/BP_Dosimeter_EPD` OtherActor))
    (if (`/Game/Game/Blueprints/Actors/Items/BP_PickableItem.Grabbed` _asbp_dosimeter_epd)
      (if (`self.Is Current Quest and Can Start` "T2004")
        (`KismetSystemLibrary.Delay` 1.0)
        (`self.CompleteQuest` (`self.CurrentQuestID`))
        (`self.SetCurrentQuest` "T2005")))))

(event `self.BindNPCActions`
  (`parent.BindNPCActions`))

(fn `UserConstructionScript`)