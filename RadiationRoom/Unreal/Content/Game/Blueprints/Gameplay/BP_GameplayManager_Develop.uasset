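; BP_GameplayManager_Develop is a gameplay manager Blueprint that extends its parent to set up the tutorial and start the scenario.
; One second after BeginPlay, it gives the TutorialManager the player's tutorial buddy actor and binds its actions, or logs if the manager is missing.
; It then calls StartScenario either way, which defers to the parent.
; SetPlayerData separately binds player actions.
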(event `self.ReceiveBeginPlay`
  (`parent.ReceiveBeginPlay`)
  (`KismetSystemLibrary.Delay` 1.0)
  (`|ExecutionSequence`
    (:`then_0`
      (bind _tutorialmanager (`self.TutorialManager`)
        (:`then`
          (`/Game/Game/Blueprints/Tutorial/BP_TutorialManager.SetCurrentTutorialBuddy` _tutorialmanager (`/Game/Game/Blueprints/Player/BP_Player_VR.TutorialBuddyActor` (`/Game/Game/FunctionLibraries/BFL_Common.GetMyPlayer`)))
          (`self.BindTuddyActions`))
        (:`else`
          (`/Game/Game/Blueprints/RR_GameInstance.Log` (`/Game/Game/FunctionLibraries/BFL_Common.GetMyGameInstance`) "NewEnumerator2" "Falta el TutorialManager" false))))
    (:`then_1`
      (`self.StartScenario`))))

(event `self.SetPlayerData`
  (`self.BindPlayerActions`))

(event `self.StartScenario`
  (`parent.StartScenario`))

(fn `UserConstructionScript`
  (`parent.UserConstructionScript`))