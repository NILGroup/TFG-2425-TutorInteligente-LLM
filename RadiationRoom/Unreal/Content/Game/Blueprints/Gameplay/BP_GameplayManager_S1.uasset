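; Gameplay manager for scenario S1, running a linear quest chain from Tuddy's intro dialog to the end of gameplay.
; Tuddy dialogs open doors, and the intro also fills quest list widgets from a DataTable.
; Room triggers, NPC conversations and completed place point managers advance the current quest.
; CompleteQuest selects each next step, enabling the tidy-up points, advancing NPC conversations and showing the end Tuddy.
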(event `self.ReceiveBeginPlay`
  (`parent.ReceiveBeginPlay`)
  (for _array_element (`self.QuestListWidget`)
    (`self.SetActorHiddenInGame` _array_element true)))

(event `self.ReceiveTick`
  (params (DeltaSeconds :type "Float (single-precision)")))

(event `self.StartScenario`
  (bind _starttuddy (`self.StartTuddy`))
  (`parent.StartScenario`)
  (`/Game/Game/Blueprints/Tutorial/BP_TutorialBuddy.Show` _starttuddy)
  (`KismetSystemLibrary.Delay` 1.0)
  (`/Game/Game/Components/AC_TuddyDialogManager.StartNewDialogByID` (`/Game/Game/Blueprints/Tutorial/BP_TutorialBuddy.AC_TuddyDialogManager` _starttuddy) "S1001"))

(event `self.CompleteQuest`
  (params (QuestID :type Name))
  (`parent.CompleteQuest` QuestID)
  (`|ExecutionSequence`
    (:`then_0`
      (switch `name` QuestID
        (:`S1001`
          (`self.SetCurrentQuest` "S1002"))
        (:`S1002`
          (`self.SetCurrentQuest` "S1003")
          (`/Game/Game/Blueprints/Characters/BP_NPC_Talkable.NextConversation` (`self.NPC`))
          (for _array_element (`self.PlacePointManagers`)
            (set `/Game/Game/Blueprints/Actors/Items/PlacePoints/BP_PlacePointManager.CanActivatePoints` true _array_element)
            (`/Game/Game/Blueprints/Actors/Items/PlacePoints/BP_PlacePointManager.ShowInfoWidget` _array_element)))
        (:`S1003`
          (`self.SetCurrentQuest` "S1004")
          (`/Game/Game/Blueprints/Characters/BP_NPC_Talkable.NextConversation` (`self.NPC`)))
        (:`S1004`
          (`self.SetCurrentQuest` "S1005")
          (`KismetSystemLibrary.Delay` 1.5)
          (`/Game/Game/Blueprints/Tutorial/BP_TutorialBuddy.Show` (`self.EndTuddy`)))
        (:`S1005`
          (`self.EndGameplay`))))
    (:`then_1`
      (if (`self.GameplayCompleted`)
        _))))

(event `self.BindTuddyActions`
  (`parent.BindTuddyActions`)
  (add `/Game/Game/Components/AC_TuddyDialogManager.ED_DialogCompleted` (`/Game/Game/Blueprints/Tutorial/BP_TutorialBuddy.AC_TuddyDialogManager` (`self.StartTuddy`)) (delegate `OnStartTuddyDialogCompleted`))
  (add `/Game/Game/Components/AC_TuddyDialogManager.ED_DialogCompleted` (`/Game/Game/Blueprints/Tutorial/BP_TutorialBuddy.AC_TuddyDialogManager` (`self.EndTuddy`)) (delegate `OnEndTuddyDialogCompleted`)))

(event `OnStartTuddyDialogCompleted`
  (params (CurrentTuddyDialogType :type "/Game/Game/DataStructures/Tutorial/E_TuddyDialogLinesType Enum" :default "NewEnumerator0") (CurrentExtraLineType :type "/Game/Game/DataStructures/Tutorial/E_TuddyExtraLineTypes Enum" :default "NewEnumerator1") (DialogID :type Name))
  (`KismetSystemLibrary.Delay` 1.0)
  (`/Game/Game/Blueprints/Tutorial/BP_TutorialBuddy.Hide` (`self.StartTuddy`))
  (`/Game/Game/Blueprints/Actors/CanOpenActors/BP_Door.AutomaticOpenAndLockDoor` (`self.BigRoomDoor`))
  (`self.SetQuestList`)
  (for _array_element (`self.QuestListWidget`)
    (`self.SetActorHiddenInGame` _array_element false))
  (`self.SetCurrentQuest` "S1001"))

(event `OnEndTuddyDialogCompleted`
  (params (CurrentTuddyDialogType :type "/Game/Game/DataStructures/Tutorial/E_TuddyDialogLinesType Enum" :default "NewEnumerator0") (CurrentExtraLineType :type "/Game/Game/DataStructures/Tutorial/E_TuddyExtraLineTypes Enum" :default "NewEnumerator1") (DialogID :type Name))
  (`KismetSystemLibrary.Delay` 0.5)
  (`/Game/Game/Blueprints/Tutorial/BP_TutorialBuddy.Hide` (`self.EndTuddy`))
  (`/Game/Game/Blueprints/Actors/CanOpenActors/BP_Door.AutomaticOpenAndLockDoor` (`self.ExitDoor`)))

(event `OnFinalConversationCompleted`
  (if (`self.Is Current Quest` "None")
    (`self.CompleteQuest` "None")))

(event `self.BindPlayerActions`
  (`parent.BindPlayerActions`)
  (add `self.OnActorBeginOverlap` (`self.BigRoomTrigger`) (delegate `OnActorEnterInBigRoom`))
  (add `self.OnActorBeginOverlap` (`self.ExitRoomTrigger`) (delegate `OnActorEnterInExitRoom`))
  (add `self.OnActorBeginOverlap` (`self.EndTuddyTrigger`) (delegate `OnActorEnterInEndTuddyTrigger`)))

(event `OnActorEnterInBigRoom` :!signature `self.OnActorBeginOverlap`
  (params (OverlappedActor :type "Actor Object Reference") (OtherActor :type "Actor Object Reference"))
  (if (`self.Is Current Quest` "S1001")
    (if (== OtherActor (`/Game/Game/FunctionLibraries/BFL_Common.GetMyPlayer`))
      (`self.CompleteQuest` "S1001"))))

(event `OnActorEnterInExitRoom`
  (params (OverlappedActor :type "Actor Object Reference") (OtherActor :type "Actor Object Reference"))
  (if (`self.Is Current Quest` "S1005")
    (if (== OtherActor (`/Game/Game/FunctionLibraries/BFL_Common.GetMyPlayer`))
      (`self.CompleteQuest` "S1005"))))

(event `OnActorEnterInEndTuddyTrigger`
  (params (OverlappedActor :type "Actor Object Reference") (OtherActor :type "Actor Object Reference"))
  (if (`self.Is Current Quest` "S1005")
    (if (== OtherActor (`/Game/Game/FunctionLibraries/BFL_Common.GetMyPlayer`))
      (`/Game/Game/Components/AC_TuddyDialogManager.StartNewDialogByID` (`/Game/Game/Blueprints/Tutorial/BP_TutorialBuddy.AC_TuddyDialogManager` (`self.EndTuddy`)) "S1002"))))

(event `self.BindPlacePointsActions`
  (`parent.BindPlacePointsActions`)
  (for _array_element (`self.PlacePointManagers`)
    (add `/Game/Game/Blueprints/Actors/Items/PlacePoints/BP_PlacePointManager.ED_AllPlacePointsWithItems` _array_element (delegate `OnPlacePointManagerCompleted`))))

(event `OnPlacePointManagerCompleted`
  (if (`self.Is Current Quest` "S1003")
    (bind _completed (`self.IsTidyUpPhaseCompleted?`))
    (if _completed
      (`self.CompleteQuest` "S1003"))))

(event `self.BindNPCActions`
  (`parent.BindNPCActions`)
  (bind _npc (`self.NPC`)
    (:`then`
      (add `/Game/Game/Blueprints/Characters/BP_NPC_Talkable.ED_ConversationFinished` _npc (delegate `OnNPCConversationFinished`)))
    (:`else`
      (`/Game/Game/Blueprints/RR_GameInstance.Log` (`/Game/Game/FunctionLibraries/BFL_Common.GetMyGameInstance`) "NewEnumerator2" "Falta NPC" false))))

(event `OnNPCConversationFinished`
  (params (ConversationNumber :type Integer))
  (switch `name` (`self.CurrentQuestID`)
    (:`S1002`
      (`self.OnNPCIntroductionCompleted`))
    (:`S1004`
      (`self.OnInformToNPCCompleted`))))

(event `OnNPCIntroductionCompleted`
  (if (`self.Is Current Quest` "S1002")
    (`self.CompleteQuest` (`self.CurrentQuestID`))))

(event `OnInformToNPCCompleted`
  (if (`self.Is Current Quest` "S1004")
    (`self.CompleteQuest` (`self.CurrentQuestID`))))

(fn `IsTidyUpPhaseCompleted?`
  (returns (Completed :type Boolean))
  (for _array_element (`self.PlacePointManagers`)
    (if (not (`/Game/Game/Blueprints/Actors/Items/PlacePoints/BP_PlacePointManager.AllPointsUsed` _array_element))
      (return false)))
  (return true))

(fn `SetQuestList`
  (locals (Quests :type "Map of Name to Text"))
  (bind _outrownames (`DataTableFunctionLibrary.GetDataTableRowNames` (`self.Quest Data Table`)))
  (for _array_element _outrownames
    (bind _returnvalue (`|GetDataTableRow` (`self.Quest Data Table`) _array_element)
      (:`then`
        (`BlueprintMapLibrary.Map_Add` (`local.Quests`) _array_element (`.TrackingDescription_43_BB4922BA4D86CE9DBF3B05BA6612A06C` (break `/Game/Game/DataStructures/Gameplay/F_GameplayStepData` _returnvalue))))))
  (for _array_element_2 (`self.QuestListWidget`)
    (`/Game/Game/Blueprints/Widgets/QuestPanels/BP_QuestList.SetQuestList` _array_element_2 (`local.Quests`))))

(fn `UserConstructionScript`)