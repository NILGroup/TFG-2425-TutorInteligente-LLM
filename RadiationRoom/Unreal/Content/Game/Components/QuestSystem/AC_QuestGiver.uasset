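; AC_QuestGiver is an actor component that lets its owner act as a quest giver in the quest system.
; On interaction it asks the player's quest log whether its configured quest is active, printing either the quest name or an "Already on Quest" notice, and returns the owner's display name.
; A lookup function fetches quest rows by name from a data table and logs through the game instance when one is missing.
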(fn `DisplayQuest`
  (bind (_questdata_datatable _questdata_rowname) (break `DataTableRowHandle` (`self.QuestData`)))
  (bind _returnvalue (`|GetDataTableRow` _questdata_datatable _questdata_rowname)
    (:`then`
      (`KismetSystemLibrary.PrintString` (`KismetTextLibrary.Conv_TextToString` (`.QuestName_2_E404055C4B3071D061ED27806DA8AFB1` (break `/Game/Game/DataStructures/QuestSystem/F_QuestDetails` _returnvalue)))))))

(fn `GetQuestByRowName`
  (params (`Row Name` :type Name))
  (returns (`Quest Data` :type "/Game/Game/DataStructures/QuestSystem/F_QuestDetails Structure"))
  (bind _returnvalue (`|GetDataTableRow` (`self.QuestDataTable`) `Row Name`)
    (:`then`
      (return _returnvalue))
    (:`RowNotFound`
      (`/Game/Game/Blueprints/RR_GameInstance.Log` (`/Game/Game/FunctionLibraries/BFL_Common.GetMyGameInstance`) "NewEnumerator2" (`|FormatText` "La quest {row_name} no existe." `Row Name`) false)
      (return))))

(fn `InteractWith`
  (returns (ObjectiveID :type String))
  (bind (_questdata_datatable _questdata_rowname) (break `DataTableRowHandle` (`self.QuestData`)))
  (bind _returnvalue (`KismetSystemLibrary.GetDisplayName` (`self.GetOwner`)))
  (if (not (`/Game/Game/Components/QuestSystem/AC_QuestLog.QueryActiveQuest` (`/Game/Game/Blueprints/Player/BP_Player.AC_QuestLog` (`/Game/Game/FunctionLibraries/BFL_Common.GetMyPlayer`)) _questdata_rowname))
    (`self.DisplayQuest`)
    (return _returnvalue)
    (else
      (`KismetSystemLibrary.PrintString` "Already on Quest")
      (return _returnvalue))))