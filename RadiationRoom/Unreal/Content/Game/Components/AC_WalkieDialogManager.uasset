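; Walkie-talkie component that plays data-table conversations between office and player through the walkie's dialog widget.
; StartConversation selects by conversation type, then each line waits its TimeToPlay before displaying as office text or three player options split on "/".
; Typewriter completion advances the dialog after a short delay, ending and signalling when no lines remain.
; Player choices are reported to the database with user, scenario, conversation type and timestamp.
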(event `self.ReceiveBeginPlay`
  (bind _asbp_walkie_talkie (cast `/Game/Game/Blueprints/WalkieTalkie/BP_WalkieTalkie` (`self.GetOwner`)))
  (set `self.Owner` _asbp_walkie_talkie))

(event `SetWalkieConversationData`
  (params (`Walkie Conversation Data` :type "DataTable Object Reference"))
  (set `self.Dialog Data Table` `Walkie Conversation Data`)
  (`self.SetDialogsFromDataTable`))

(event `self.ReceiveTick`
  (params (DeltaSeconds :type "Float (single-precision)")))

(event `Interact With`
  ;[1 1 1] Interact with
  (if (not (`self.IsTalking?`))
    (`SceneComponent.SetHiddenInGame` (`self.Widget Component`) false false)
    (`/Game/Game/UserInterfaces/Items/WalkieTalkie/WBP_WalkieTalkie.ShowDialogBox` (`self.Widget Actor`))))

(event `CancelInteract`
  ;[1 1 1] Interact with
  (if (not (`self.IsTalking?`))
    (`SceneComponent.SetHiddenInGame` (`self.Widget Component`) true false)
    (`/Game/Game/UserInterfaces/Items/WalkieTalkie/WBP_WalkieTalkie.HideDialogBox` (`self.Widget Actor`))))

(event `StartConversation`
  (params (WalkieConversationType :type "/Game/Game/DataStructures/Walkie/E_WalkieConversationType Enum" :default "NewEnumerator0"))
  ;[1 1 1] Conversation
  (set `self.CurrentWalkieConversationType` WalkieConversationType)
  (bind _isempty (`self.Is Conversation Empty`))
  (if (and (not _isempty) (`self.CanStartConversation?`))
    (set `self.IsTalking?` true)
    (set `self.DialogIndex` 0)
    (`self.ProcessDialog`)
    (`SceneComponent.SetHiddenInGame` (`self.Widget Component`) false false)
    (`/Game/Game/UserInterfaces/Items/WalkieTalkie/WBP_WalkieTalkie.ShowDialogBox` (`self.Widget Actor`))))

(event `StopConversation`
  ;[1 1 1] Conversation
  (set `self.IsTalking?` false)
  (`self.ConversationFinished` (`self.CurrentWalkieConversationType`))
  (`SceneComponent.SetHiddenInGame` (`self.Widget Component`) true false)
  (`/Game/Game/UserInterfaces/Items/WalkieTalkie/WBP_WalkieTalkie.HideDialogBox` (`self.Widget Actor`)))

(event `ContinueDialog`
  ;[1 1 1] Process Dialog
  (`self.ProcessDialog`))

(event `ProcessDialog`
  ;[1 1 1] Process Dialog
  (if (`self.IsTalking?`)
    (bind _dialog (`self.GetCurrentDialog`))
    (bind (_type _text _timetoplay) (break `/Game/Game/DataStructures/Walkie/F_WalkieLine` _dialog))
    (`KismetSystemLibrary.Delay` _timetoplay)
    (switch `/Game/Game/DataStructures/Dialogs/E_DialogType` _type
      (:`NewEnumerator2`
        (`KismetSystemLibrary.PrintString` "Un diálogo que no tiene dueño :(" true true (struct :`R` 1.0 :`A` 1.0)))
      (:`NewEnumerator4`
        (`self.CreatePlayerDialog`))
      (:`NewEnumerator5`
        (`self.CreateOfficeDialog`)))))

(event `SetTypewriterComponent`
  (params (TypewriterComponent :type "TypewriterTextComponent Object Reference"))
  (bind _output_get (set `self.TypewriterComponent` TypewriterComponent))
  (add `TypewriterTextComponent.OnCompleted` _output_get (delegate `OnTypewriterFinished`)))

(event `OnTypewriterFinished`
  (`KismetSystemLibrary.Delay` 1.0)
  (if (`self.IsTalking?`)
    (bind _continue (`self.Next Dialog`))
    (if _continue
      (`self.ProcessDialog`)
      (else
        (`self.StopConversation`)))))

(event `SetWidgetComponent`
  (params (WidgetComponent :type "WidgetComponent Object Reference") (WidgetActor :type "/Game/Game/UserInterfaces/Items/WalkieTalkie/WBP_WalkieTalkie Object Reference"))
  (set `self.Widget Component` WidgetComponent)
  (bind _output_get (set `self.Widget Actor` WidgetActor))
  (add `/Game/Game/UserInterfaces/Items/WalkieTalkie/WBP_WalkieTalkie.ED_OnPlayerOptionSelected` _output_get (delegate `OnPlayerOptionSelected`))
  (`SceneComponent.SetHiddenInGame` (`self.Widget Component`) false false))

(event `OnPlayerOptionSelected`
  (params (PlayerDialogIndex :type Integer) (OptionSelectedIndex :type Integer))
  (`self.SendReportEventToDataBase` PlayerDialogIndex OptionSelectedIndex))

(fn `CreateOfficeDialog`
  (bind _dialog (`self.GetCurrentDialog`))
  (`/Game/Game/UserInterfaces/Items/WalkieTalkie/WBP_WalkieTalkie.CreateWalkieOfficeText` (`self.Widget Actor`) (`.Text_2_8889C3EB4A46B35524B709947C974DCC` (break `/Game/Game/DataStructures/Walkie/F_WalkieLine` _dialog))))

(fn `CreatePlayerDialog`
  (bind _dialog (`self.GetCurrentDialog`))
  (bind (_lefts _rights) (`KismetStringLibrary.Split` (`KismetTextLibrary.Conv_TextToString` (`.Text_2_8889C3EB4A46B35524B709947C974DCC` (break `/Game/Game/DataStructures/Walkie/F_WalkieLine` _dialog))) "/"))
  (bind (_lefts_2 _rights_2) (`KismetStringLibrary.Split` _rights "/"))
  (`/Game/Game/UserInterfaces/Items/WalkieTalkie/WBP_WalkieTalkie.CreateWalkiePlayerText` (`self.Widget Actor`) (`self.CurrentUserDialogIndex`) (`KismetTextLibrary.Conv_StringToText` _lefts) (`KismetTextLibrary.Conv_StringToText` _lefts_2) (`KismetTextLibrary.Conv_StringToText` _rights_2))
  (bind _result (`/Engine/EditorBlueprintResources/StandardMacros.IncrementInt` (`self.CurrentUserDialogIndex`))
    (:`  `
      (set `self.CurrentUserDialogIndex` _result))))

(fn `GetCurrentConversation`
  (returns (CurrentConversation :type "/Game/Game/DataStructures/Walkie/F_WalkieConversation Structure (by ref)"))
  (for _array_element (`self.Conversations`)
    (if (`|EnumEquality` (`self.CurrentWalkieConversationType`) (`.ConversationType_45_4DF166FC44BB30C452EE3A9E4EDC0375` (break `/Game/Game/DataStructures/Walkie/F_WalkieConversation` _array_element)))
      (return _array_element))))

(fn `GetCurrentDialog`
  (returns (Dialog :type "/Game/Game/DataStructures/Walkie/F_WalkieLine Structure"))
  (bind _currentconversation (`self.GetCurrentConversation`))
  (return (`|GetArrayItem` (`.DialogData_43_CA31413047BF35DEDAF362AFEAA84133` (break `/Game/Game/DataStructures/Walkie/F_WalkieConversation` _currentconversation)) (`self.DialogIndex`))))

(fn `Is Conversation Empty`
  (returns (IsEmpty :type Boolean))
  (return (== (`KismetArrayLibrary.Array_Length` (`self.Conversations`)) 0)))

(fn `Next Dialog`
  (returns (Continue :type Boolean))
  (bind _currentconversation (`self.GetCurrentConversation`))
  (bind _returnvalue (`KismetArrayLibrary.Array_Length` (`.DialogData_43_CA31413047BF35DEDAF362AFEAA84133` (break `/Game/Game/DataStructures/Walkie/F_WalkieConversation` _currentconversation))))
  (if (and (> _returnvalue 0) (< (+ (`self.DialogIndex`) 1) _returnvalue))
    (`/Engine/EditorBlueprintResources/StandardMacros.IncrementInt` (`self.DialogIndex`)
      (:`  `
        (return true)))
    (else
      (return false))))

(fn `SendReportEventToDataBase`
  (params (QuestionIndex :type Integer) (AnswerIndex :type Integer))
  (bind _database_manager (`/Game/Game/FunctionLibraries/BFL_Common.GetMyDatabase`))
  (bind _data (`/Game/Game/Blueprints/RR_GameInstance.GetDataBaseMainInfoEvent` (`/Game/Game/FunctionLibraries/BFL_Common.GetMyGameInstance`)))
  (`/Engine/EditorBlueprintResources/StandardMacros.IsValid` _database_manager
    (:`Is Valid`
      (bind (_user_id _scenario_type) (break `/Game/Game/DataStructures/Database/F_MainInfoEvent` _data))
      (`/Game/Game/Blueprints/Database/BP_DataBase_Manager.Send WalkieReport Event To DB` _database_manager (make `/Game/Game/DataStructures/Database/F_WalkieReportEvent` 0 _user_id _scenario_type (`self.CurrentWalkieConversationType`) QuestionIndex AnswerIndex (`KismetMathLibrary.Now`))))))

(fn `SetDialogsFromDataTable`
  (`KismetArrayLibrary.Array_Clear` (`self.Conversations`))
  (bind _dialog_data_table (`self.Dialog Data Table`)
    (:`then`
      (bind _outrownames (`DataTableFunctionLibrary.GetDataTableRowNames` _dialog_data_table))
      (for _array_element _outrownames
        (bind _returnvalue (`|GetDataTableRow` _dialog_data_table _array_element)
          (:`then`
            (`KismetArrayLibrary.Array_Add` (`self.Conversations`) _returnvalue)))))
    (:`else`)))